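; Networked stat manager that stores named float, int and string stats in parallel name/value arrays.
; Shared macros read or upsert values, and changes fire per-type events.
; ClientStatSetRouting applies changes on the server, while clients send RPCs for whitelisted names and optionally change values locally.
; IncrementFloatStat looks up FloatStats through IntStatNames, unlike the other float accessors, which use FloatStatNames.
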(event `ServerRequestSetFloatStat`
  (params (StatName :type Name) (StatValue :type "Float (double-precision)"))
  ;[1 1 1] Float Networking
  (if (`self.CanClientSetStat` StatName)
    (`self.SetFloatStat` StatName StatValue)))

(event `ServerRequestIncrementFloatStat`
  (params (StatName :type Name) (StatValue :type "Float (double-precision)"))
  ;[1 1 1] Float Networking
  (if (`self.CanClientSetStat` StatName)
    (`self.IncrementFloatStat` StatName StatValue)))

(event `ServerRequestSetIntStat`
  (params (StatName :type Name) (StatValue :type Integer))
  ;[1 1 1] Int Networking
  (if (`self.CanClientSetStat` StatName)
    (`self.SetIntStat` StatName StatValue)))

(event `ServerRequestIncrementIntStat`
  (params (StatName :type Name) (StatValue :type Integer))
  ;[1 1 1] Int Networking
  (if (`self.CanClientSetStat` StatName)
    (`self.IncrementIntStat` StatName StatValue)))

(event `ServerRequestSetStringStat`
  (params (StatName :type Name) (StatValue :type String))
  ;[1 1 1] String Networking
  (if (`self.CanClientSetStat` StatName)
    (`self.SetStringStat` StatName StatValue)))

(fn `CanClientSetStat`
  (params (StatName :type Name))
  (returns (bCanSet :type Boolean))
  (return (`BlueprintSetLibrary.Set_Contains` (`self.ClientSettableStatNames`) StatName)))

(fn `GetFloatStat`
  (params (StatName :type Name) (DefaultValue :type "Float (double-precision)"))
  (returns (StatValue :type "Float (double-precision)"))
  (bind _statvalue (`self.GetStatValue` StatName DefaultValue (`self.FloatStatNames`) (`self.FloatStats`)))
  (return _statvalue))

(fn `GetIntStat`
  (params (StatName :type Name) (DefaultValue :type Integer))
  (returns (StatValue :type Integer))
  (bind _statvalue (`self.GetStatValue` StatName DefaultValue (`self.IntStatNames`) (`self.IntStats`)))
  (return _statvalue))

(fn `GetStringStat`
  (params (StatName :type Name) (DefaultValue :type String))
  (returns (StatValue :type String))
  (bind _statvalue (`self.GetStatValue` StatName DefaultValue (`self.StringStatNames`) (`self.StringStats`)))
  (return _statvalue))

(fn `IncrementFloatStat`
  (params (StatName :type Name) (Amount :type "Float (double-precision)"))
  (returns (NewValue :type "Float (double-precision)"))
  (locals (NewFloatValue :type "Float (double-precision)"))
  (`self.ClientStatSetRouting` StatName
    (:`DoStatChange`
      (bind _statvalue (`self.GetStatValue` StatName 0.0 (`self.IntStatNames`) (`self.FloatStats`)))
      (bind _output_get (set `local.NewFloatValue` (+ _statvalue Amount)))
      (`self.SetStatValue` StatName _output_get (`self.IntStatNames`) (`self.FloatStats`))
      (`self.OnFloatStatChanged` StatName (`local.NewFloatValue`))
      (return (`local.NewFloatValue`)))
    (:`DoServerRPC`
      (`self.ServerRequestIncrementFloatStat` StatName Amount))
    (:`DontClientsideChange`
      (return 0.0))))

(fn `IncrementIntStat`
  (params (StatName :type Name) (Amount :type Integer))
  (returns (NewValue :type Integer))
  (locals (NewIntValue :type Integer))
  (bind _newintvalue (`local.NewIntValue`))
  (`self.ClientStatSetRouting` StatName
    (:`DoStatChange`
      (bind _statvalue (`self.GetStatValue` StatName 0 (`self.IntStatNames`) (`self.IntStats`)))
      (bind _output_get (set `local.NewIntValue` (+ _statvalue Amount)))
      (`self.SetStatValue` StatName _output_get (`self.IntStatNames`) (`self.IntStats`))
      (`self.OnIntStatChanged` StatName _newintvalue)
      (return _newintvalue))
    (:`DoServerRPC`
      (`self.ServerRequestIncrementIntStat` StatName Amount))
    (:`DontClientsideChange`
      (return 0))))

(fn `SetFloatStat`
  (params (StatValue :type Name) (NewValue :type "Float (double-precision)"))
  (returns (bWasNewlyAdded :type Boolean))
  (locals (bAdded :type Boolean))
  (`self.ClientStatSetRouting` StatValue
    (:`DoStatChange`
      (bind _boutwasnewlyadded (`self.SetStatValue` StatValue NewValue (`self.FloatStatNames`) (`self.FloatStats`)))
      (`self.OnFloatStatChanged` StatValue NewValue)
      (return _boutwasnewlyadded))
    (:`DoServerRPC`
      (`self.ServerRequestSetFloatStat` StatValue NewValue))
    (:`DontClientsideChange`
      (return false))))

(fn `SetIntStat`
  (params (StatName :type Name) (NewValue :type Integer))
  (returns (bWasNewlyAdded :type Boolean))
  (locals (bAdded :type Boolean))
  (`self.ClientStatSetRouting` StatName
    (:`DoStatChange`
      (bind _boutwasnewlyadded (`self.SetStatValue` StatName NewValue (`self.IntStatNames`) (`self.IntStats`)))
      (`self.OnIntStatChanged` StatName NewValue)
      (return _boutwasnewlyadded))
    (:`DoServerRPC`
      (`self.ServerRequestSetIntStat` StatName NewValue))
    (:`DontClientsideChange`
      (return false))))

(fn `SetStringStat`
  (params (StatName :type Name) (StatValue :type String))
  (returns (bWasNewlyAdded :type Boolean))
  (locals (bAdded :type Boolean))
  (`self.ClientStatSetRouting` StatName
    (:`DoStatChange`
      (bind _boutwasnewlyadded (`self.SetStatValue` StatName StatValue (`self.StringStatNames`) (`self.StringStats`)))
      (`self.OnStringStatChanged` StatName StatValue)
      (return _boutwasnewlyadded))
    (:`DoServerRPC`
      (`self.ServerRequestSetStringStat` StatName StatValue))
    (:`DontClientsideChange`
      (return false))))