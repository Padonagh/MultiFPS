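; Settings bucket for audio that stores per-sound-class volumes and applies them through a master sound mix.
; ApplySettings gets a temporary settings helper, sets the base mix, pushes each stored volume as a sound class override, then destroys the helper.
; SetVolume updates the map, reapplies all settings and optionally saves, while GetVolume looks up a class's volume and reports whether it was found.
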(fn `ApplySettings`
  (returns (bApplied :type Boolean))
  (locals (Helper :type "/Game/GenericShooter/Addons/SettingsManager/Core/BP_SettingsManagerHelper Object Reference"))
  (bind _volumes (`self.Volumes`))
  (bind _helper (`self.GetTemporarySettingsHelper`))
  (bind _output_get (set `local.Helper` _helper))
  (`/Game/GenericShooter/Addons/SettingsManager/Core/BP_SettingsManagerHelper.SetBaseSoundMix` _output_get (`self.SoundMixMaster`))
  (bind _keys (`BlueprintMapLibrary.Map_Keys` _volumes))
  (bind _values (`BlueprintMapLibrary.Map_Values` _volumes))
  (for (_array_element _array_index) _keys
    (`/Game/GenericShooter/Addons/SettingsManager/Core/BP_SettingsManagerHelper.SetSoundMixVolumeOverride` (`local.Helper`) (`self.SoundMixMaster`) (`|GetArrayItem` _values _array_index) _array_element))
  (`Actor.K2_DestroyActor` (`local.Helper`))
  (return true))

(fn `GetVolume`
  (params (SoundClassName :type Name))
  (returns (Volume :type "Float (double-precision)") (bFound :type Boolean))
  (bind (_value _returnvalue) (`BlueprintMapLibrary.Map_Find` (`self.Volumes`) SoundClassName))
  (return _value _returnvalue))

(fn `SetVolume`
  (params (SoundClassName :type Name) (Volume :type "Float (double-precision)" :default 1.0) (bSave :type Boolean :default true))
  (returns (bVolumeSet :type Boolean))
  (`BlueprintMapLibrary.Map_Add` (`self.Volumes`) SoundClassName Volume)
  (`self.ApplySettings`)
  (if (`local.bSave`)
    (`self.SaveCurrent`))
  (return true))