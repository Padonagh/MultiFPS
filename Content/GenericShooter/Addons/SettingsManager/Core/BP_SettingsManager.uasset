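; BP_SettingsManager loads, creates and applies the game's settings, grouped into named buckets stored as save game objects.
; On Initialize, each bucket class loads from a slot named by prefix plus bucket name, or is created and saves its defaults, then is applied.
; Buckets receive a manager back-reference and are retrievable by name or class.
; A temporary helper is fetched through a Game Instance message call.
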(fn `GetBucketByClass`
  (params (BucketClass :type "/Game/GenericShooter/Addons/SettingsManager/Core/BP_SettingsBucket_Base Class Reference"))
  (returns (Bucket :type "/Game/GenericShooter/Addons/SettingsManager/Core/BP_SettingsBucket_Base Object Reference"))
  (bind _values (`BlueprintMapLibrary.Map_Values` (`self.Buckets`)))
  (for _array_element _values
    (if (== (`GameplayStatics.GetObjectClass` _array_element) (`local.BucketClass`))
      (return _array_element)))
  (return null))

(fn `GetBucketByName`
  (params (BucketName :type Name))
  (returns (Bucket :type "/Game/GenericShooter/Addons/SettingsManager/Core/BP_SettingsBucket_Base Object Reference"))
  (return (`BlueprintMapLibrary.Map_Find` (`self.Buckets`) BucketName)))

(fn `GetTemporarySettingsManagerHelper`
  (returns (Helper :type "/Game/GenericShooter/Addons/SettingsManager/Core/BP_SettingsManagerHelper Object Reference"))
  (bind _gameinstance (`self.GameInstance`)
    (:`then`
      (bind _helper (message `/Game/GenericShooter/Addons/SettingsManager/Core/BPI_SettingsManagerHolder.GetTemporarySettingsManagerHelper` _gameinstance))
      (return _helper))
    (:`else`
      (`KismetSystemLibrary.PrintString` null "ERROR: Settings Manager can't get temporary settings helper because Game Instance is invalid!" true true (struct :`R` 1.0 :`G` 0.015914 :`A` 1.0) 10.0)
      (return null))))

(fn `Initialize`
  (`BlueprintMapLibrary.Map_Clear` (`self.Buckets`))
  (for _array_element (`self.BucketClasses`)
    (bind _returnvalue (`GameplayStatics.LoadGameFromSlot` (`KismetStringLibrary.Concat_StrStr` (`self.SaveSlotPrefix`) (`KismetStringLibrary.Conv_NameToString` (defaults `/Game/GenericShooter/Addons/SettingsManager/Core/BP_SettingsManager` _array_element)))))
    (bind _asbp_settings_bucket_base (cast `/Game/GenericShooter/Addons/SettingsManager/Core/BP_SettingsBucket_Base` _returnvalue)
      (:`then`
        (set `/Game/GenericShooter/Addons/SettingsManager/Core/BP_SettingsBucket_Base.SettingsManager` self _asbp_settings_bucket_base)
        (`BlueprintMapLibrary.Map_Add` (`self.Buckets`) (`/Game/GenericShooter/Addons/SettingsManager/Core/BP_SettingsBucket_Base.BucketName` _asbp_settings_bucket_base) _asbp_settings_bucket_base)
        (`/Game/GenericShooter/Addons/SettingsManager/Core/BP_SettingsBucket_Base.ApplySettings` _asbp_settings_bucket_base))
      (:`CastFailed`
        (bind _returnvalue_2 (`GameplayStatics.CreateSaveGameObject` _array_element))
        (set `/Game/GenericShooter/Addons/SettingsManager/Core/BP_SettingsBucket_Base.SettingsManager` self _returnvalue_2)
        (`/Game/GenericShooter/Addons/SettingsManager/Core/BP_SettingsBucket_Base.SaveDefaults` _returnvalue_2 (`self.SaveSlotPrefix`))
        (`BlueprintMapLibrary.Map_Add` (`self.Buckets`) (`/Game/GenericShooter/Addons/SettingsManager/Core/BP_SettingsBucket_Base.BucketName` _returnvalue_2) _returnvalue_2)
        (`/Game/GenericShooter/Addons/SettingsManager/Core/BP_SettingsBucket_Base.ApplySettings` _returnvalue_2))))
  (return))