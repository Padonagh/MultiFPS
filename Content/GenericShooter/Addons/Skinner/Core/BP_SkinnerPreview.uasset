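; BP_SkinnerPreview is a preview actor in the Skinner addon that shows an optional skeletal mesh attached to its third-person mesh.
; When a preview attach mesh is valid, the construction script creates a skeletal mesh component for it and applies the optional AnimBP.
; The component snaps to the configured socket on ThirdPersonMesh, keeps world scale, then takes the configured relative location and rotation offsets.
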(fn `UserConstructionScript`
  (`self.PreviewAttachMesh`
    (:`then`
      (bind _returnvalue (`AddComponent|NODE_AddSkeletalMeshComponent-0` :`bManualAttachment` true))
      (`SkinnedMeshComponent.SetSkinnedAssetAndUpdate` _returnvalue (`self.PreviewAttachMesh`) true)
      (bind _previewattachmeshanimbp (`self.PreviewAttachMeshAnimBP`)
        (:`then`
          (`SkeletalMeshComponent.SetAnimInstanceClass` _returnvalue _previewattachmeshanimbp))
        (:`else`
          _))
      (`SceneComponent.K2_AttachToComponent` _returnvalue (`self.ThirdPersonMesh`) (`self.PreviewAttachSocket`) "SnapToTarget" "SnapToTarget" "KeepWorld" true)
      (`SceneComponent.K2_SetRelativeLocationAndRotation` _returnvalue (`self.PreviewAttachLocationOffset`) (`self.PreviewAttachRotationOffset`) false false))
    (:`else`)))