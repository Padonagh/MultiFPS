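; Replicated component that stores named int, float and string stats with get, set and increment (numeric only) functions.
; Each type uses parallel name and value arrays, adding missing names on set and broadcasting change events.
; A routing macro applies changes on the server, while clients send RPCs only for whitelisted stat names and can optionally change values locally.
; RepNotifies broadcast changes only when name and value array lengths match.
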(event `self.ReceiveBeginPlay`
  (`|ExecutionSequence`
    (:`then_0`
      ;[1 1 1] Ensure Int Stats are synced
      (if (!= (`KismetArrayLibrary.Array_Length` (`self.IntStatNames`)) (`KismetArrayLibrary.Array_Length` (`self.IntStats`)))
        (`KismetSystemLibrary.PrintString` "ERROR: BP_StatManager started with mismatch between Int Stat Names and Int Stat Values!" true true (struct :`R` 1.0 :`G` 0.033889 :`A` 1.0) 5.0)
        (`KismetArrayLibrary.Array_Resize` (`self.IntStats`) (`KismetArrayLibrary.Array_Length` (`self.IntStatNames`)))))
    (:`then_1`
      ;[1 1 1] Ensure Float Stats are synced
      (if (!= (`KismetArrayLibrary.Array_Length` (`self.FloatStatNames`)) (`KismetArrayLibrary.Array_Length` (`self.FloatStats`)))
        (`KismetSystemLibrary.PrintString` "ERROR: BP_StatManager started with mismatch between Int Stat Names and Float Stat Values!" true true (struct :`R` 1.0 :`G` 0.033889 :`A` 1.0) 5.0)
        (`KismetArrayLibrary.Array_Resize` (`self.FloatStats`) (`KismetArrayLibrary.Array_Length` (`self.FloatStatNames`)))))
    (:`then_2`
      ;[1 1 1] Ensure String Stats are synced
      (if (!= (`KismetArrayLibrary.Array_Length` (`self.StringStatNames`)) (`KismetArrayLibrary.Array_Length` (`self.StringStats`)))
        (`KismetSystemLibrary.PrintString` "ERROR: BP_StatManager started with mismatch between Int Stat Names and String Stat Values!" true true (struct :`R` 1.0 :`G` 0.033889 :`A` 1.0) 5.0)
        (`KismetArrayLibrary.Array_Resize` (`self.StringStats`) (`KismetArrayLibrary.Array_Length` (`self.StringStatNames`)))))))

(event `ServerRequestSetFloatStat`
  (params (StatName :type Name) (StatValue :type "Float (double-precision)"))
  ;[1 1 1] Float Networking
  (bind _bcanset (`self.CanClientSetStat` StatName))
  (if _bcanset
    (`self.SetFloatStat` StatName StatValue)))

(event `ServerRequestIncrementFloatStat`
  (params (StatName :type Name) (StatValue :type "Float (double-precision)"))
  ;[1 1 1] Float Networking
  (bind _bcanset (`self.CanClientSetStat` StatName))
  (if _bcanset
    (`self.IncrementFloatStat` StatName StatValue)))

(event `ServerRequestSetIntStat`
  (params (StatName :type Name) (StatValue :type Integer))
  ;[1 1 1] Int Networking
  (bind _bcanset (`self.CanClientSetStat` StatName))
  (if _bcanset
    (`self.SetIntStat` StatName StatValue)))

(event `ServerRequestIncrementIntStat`
  (params (StatName :type Name) (StatValue :type Integer))
  ;[1 1 1] Int Networking
  (bind _bcanset (`self.CanClientSetStat` StatName))
  (if _bcanset
    (`self.IncrementIntStat` StatName StatValue)))

(event `ServerRequestSetStringStat`
  (params (StatName :type Name) (StatValue :type String))
  ;[1 1 1] String Networking
  (bind _bcanset (`self.CanClientSetStat` StatName))
  (if _bcanset
    (`self.SetStringStat` StatName StatValue)))

(fn `CanClientSetStat`
  (params (StatName :type Name))
  (returns (bCanSet :type Boolean))
  (return (`BlueprintSetLibrary.Set_Contains` (`self.ClientSettableStatNames`) StatName)))

(fn `GetAllStoredFloatStats`
  (returns (OutFloatStatNames :type "Array of Name") (OutFloatStatValues :type "Array of Float (double-precision)"))
  (return (`self.FloatStatNames`) (`self.FloatStats`)))

(fn `GetAllStoredIntStats`
  (returns (OutIntStatNames :type "Array of Name") (OutIntStatValues :type "Array of Integer"))
  (return (`self.IntStatNames`) (`self.IntStats`)))

(fn `GetAllStoredStringStats`
  (returns (OutStringStatNames :type "Array of Name") (OutStringStatValues :type "Array of String"))
  (return (`self.StringStatNames`) (`self.StringStats`)))

(fn `GetFloatStat`
  (params (StatName :type Name) (DefaultValue :type "Float (double-precision)"))
  (returns (StatValue :type "Float (double-precision)"))
  (bind _statvalue (`self.GetStatValue` StatName DefaultValue (`self.FloatStatNames`) (`self.FloatStats`)))
  (return _statvalue))

(fn `GetIntStat`
  (params (StatName :type Name) (DefaultValue :type Integer))
  (returns (StatValue :type Integer))
  (bind _statvalue (`self.GetStatValue` StatName DefaultValue (`self.IntStatNames`) (`self.IntStats`)))
  (return _statvalue))

(fn `GetStringStat`
  (params (StatName :type Name) (DefaultValue :type String))
  (returns (StatValue :type String))
  (bind _statvalue (`self.GetStatValue` StatName DefaultValue (`self.StringStatNames`) (`self.StringStats`)))
  (return _statvalue))

(fn `IncrementFloatStat`
  (params (StatName :type Name) (Amount :type "Float (double-precision)"))
  (returns (NewValue :type "Float (double-precision)"))
  (locals (NewFloatValue :type "Float (double-precision)") (LocalStatName :type Name))
  (bind _output_get (set `local.LocalStatName` StatName))
  (`self.ClientStatSetRouting` _output_get
    (:`DoStatChange`
      (bind _statvalue (`self.GetStatValue` (`local.LocalStatName`) 0.0 (`self.FloatStatNames`) (`self.FloatStats`)))
      (bind _output_get_2 (set `local.NewFloatValue` (+ _statvalue Amount)))
      (`self.SetStatValue` (`local.LocalStatName`) _output_get_2 (`self.FloatStatNames`) (`self.FloatStats`))
      (`self.OnExplicitFloatStatChanged` (`local.LocalStatName`) (`local.NewFloatValue`))
      (`self.OnAnyStatChanged`)
      (return (`local.NewFloatValue`)))
    (:`DoServerRPC (Do Not Return)`
      (`self.ServerRequestIncrementFloatStat` (`local.LocalStatName`) Amount))
    (:`DontClientsideChange`
      (return 0.0))))

(fn `IncrementIntStat`
  (params (StatName :type Name) (Amount :type Integer))
  (returns (NewValue :type Integer))
  (locals (NewIntValue :type Integer) (LocalStatName :type Name))
  (bind _newintvalue (`local.NewIntValue`))
  (bind _output_get (set `local.LocalStatName` StatName))
  (`self.ClientStatSetRouting` _output_get
    (:`DoStatChange`
      (bind _statvalue (`self.GetStatValue` (`local.LocalStatName`) 0 (`self.IntStatNames`) (`self.IntStats`)))
      (bind _output_get_2 (set `local.NewIntValue` (+ _statvalue Amount)))
      (`self.SetStatValue` (`local.LocalStatName`) _output_get_2 (`self.IntStatNames`) (`self.IntStats`))
      (`self.OnExplicitIntStatChanged` (`local.LocalStatName`) _newintvalue)
      (`self.OnAnyStatChanged`)
      (return _newintvalue))
    (:`DoServerRPC (Do Not Return)`
      (`self.ServerRequestIncrementIntStat` (`local.LocalStatName`) Amount))
    (:`DontClientsideChange`
      (return 0))))

(fn `OnRep_FloatStatNames`
  (if (== (`KismetArrayLibrary.Array_Length` (`self.FloatStatNames`)) (`KismetArrayLibrary.Array_Length` (`self.FloatStats`)))
    (`self.OnAnyStatChanged`)
    (return)
    (else
      (return))))

(fn `OnRep_FloatStats`
  (if (== (`KismetArrayLibrary.Array_Length` (`self.FloatStatNames`)) (`KismetArrayLibrary.Array_Length` (`self.FloatStats`)))
    (`self.OnAnyStatChanged`)
    (return)
    (else
      (return))))

(fn `OnRep_IntStatNames`
  (if (== (`KismetArrayLibrary.Array_Length` (`self.IntStatNames`)) (`KismetArrayLibrary.Array_Length` (`self.IntStats`)))
    (`self.OnAnyStatChanged`)
    (return)
    (else
      (return))))

(fn `OnRep_IntStats`
  (if (== (`KismetArrayLibrary.Array_Length` (`self.IntStatNames`)) (`KismetArrayLibrary.Array_Length` (`self.IntStats`)))
    (`self.OnAnyStatChanged`)
    (return)
    (else
      (return))))

(fn `OnRep_StringStatNames`
  (if (== (`KismetArrayLibrary.Array_Length` (`self.StringStatNames`)) (`KismetArrayLibrary.Array_Length` (`self.StringStats`)))
    (`self.OnAnyStatChanged`)
    (return)
    (else
      (return))))

(fn `OnRep_StringStats`
  (if (== (`KismetArrayLibrary.Array_Length` (`self.StringStatNames`)) (`KismetArrayLibrary.Array_Length` (`self.StringStats`)))
    (`self.OnAnyStatChanged`)
    (return)
    (else
      (return))))

(fn `SetFloatStat`
  (params (StatValue :type Name) (NewValue :type "Float (double-precision)"))
  (returns (bWasNewlyAdded :type Boolean))
  (locals (bAdded :type Boolean))
  (`self.ClientStatSetRouting` StatValue
    (:`DoStatChange`
      (bind _boutwasnewlyadded (`self.SetStatValue` StatValue NewValue (`self.FloatStatNames`) (`self.FloatStats`)))
      (`self.OnExplicitFloatStatChanged` StatValue NewValue)
      (`self.OnAnyStatChanged`)
      (return _boutwasnewlyadded))
    (:`DoServerRPC (Do Not Return)`
      (`self.ServerRequestSetFloatStat` StatValue NewValue))
    (:`DontClientsideChange`
      (return false))))

(fn `SetIntStat`
  (params (StatName :type Name) (NewValue :type Integer))
  (returns (bWasNewlyAdded :type Boolean))
  (locals (bAdded :type Boolean) (LocalStatName :type Name))
  (set `local.LocalStatName` StatName)
  (`self.ClientStatSetRouting` (`local.LocalStatName`)
    (:`DoStatChange`
      (bind _boutwasnewlyadded (`self.SetStatValue` (`local.LocalStatName`) NewValue (`self.IntStatNames`) (`self.IntStats`)))
      (`self.OnExplicitIntStatChanged` (`local.LocalStatName`) NewValue)
      (`self.OnAnyStatChanged`)
      (return _boutwasnewlyadded))
    (:`DoServerRPC (Do Not Return)`
      (`self.ServerRequestSetIntStat` (`local.LocalStatName`) NewValue))
    (:`DontClientsideChange`
      (return false))))

(fn `SetStringStat`
  (params (StatName :type Name) (StatValue :type String))
  (returns (bWasNewlyAdded :type Boolean))
  (locals (bAdded :type Boolean) (LocalStatName :type Name))
  (bind _output_get (set `local.LocalStatName` StatName))
  (`self.ClientStatSetRouting` _output_get
    (:`DoStatChange`
      (bind _boutwasnewlyadded (`self.SetStatValue` (`local.LocalStatName`) StatValue (`self.StringStatNames`) (`self.StringStats`)))
      (`self.OnExplicitStatChanged` (`local.LocalStatName`) StatValue)
      (`self.OnAnyStatChanged`)
      (return _boutwasnewlyadded))
    (:`DoServerRPC (Do Not Return)`
      (`self.ServerRequestSetStringStat` (`local.LocalStatName`) StatValue))
    (:`DontClientsideChange`
      (return false))))