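; Slot-based inventory component that holds item info actors and drives a weapon-bar widget for slot selection.
; Added items are validated by the item itself, then kept priority-sorted, with OnRep refreshing the bar created for locally controlled characters.
; Slot switching cycles items within a slot, then commits immediately with FastSwitch or awaits CommitToSelected.
; Removal can pick a replacement selection, and events report item changes to listeners.
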(event `self.ReceiveBeginPlay`
  (`self.CreateWeaponBarWidget`))

(event `self.ReceiveEndPlay`
  (params (EndPlayReason :type "EEndPlayReason Enum" :default "Destroyed"))
  (`self.Cleanup` false))

(fn `AddItem`
  (params (NewItem :type "/Game/GenericShooter/Addons/Common/Blueprints/BaseClasses/BP_SlotInventory_ItemInfo_Base Object Reference") (bRebuildBar :type Boolean :default true))
  (returns (bAdded :type Boolean))
  (bind _iteminfos (`self.ItemInfos`))
  (if (`self.CanAddItem` NewItem)
    (`KismetArrayLibrary.Array_Add` _iteminfos (`local.NewItem`))
    (`self.SortItemsByPriority`)
    (bind _weaponbarwidget (`self.WeaponBarWidget`)
      (:`then`
        (set `/Game/GenericShooter/Addons/SlotInventory/Core/UI/WBP_SlotInventory.ItemReferences` _iteminfos _weaponbarwidget)
        (if (`local.bRebuildBar`)
          (`/Game/GenericShooter/Addons/SlotInventory/Core/UI/WBP_SlotInventory.BuildSlots` _weaponbarwidget)))
      (:`else`
        _))
    (`self.OnItemAdded` (`local.NewItem`))
    (return true)
    (else
      (return false))))

(fn `AddItemFromItemInfoClass`
  (params (NewItemInfoClass :type "/Game/GenericShooter/Addons/Common/Blueprints/BaseClasses/BP_SlotInventory_ItemInfo_Base Class Reference") (bRebuildBar :type Boolean :default true))
  (returns (NewItemInfo :type "/Game/GenericShooter/Addons/Common/Blueprints/BaseClasses/BP_SlotInventory_ItemInfo_Base Object Reference") (bAdded :type Boolean))
  (locals (LocalNewItemInfo :type "/Game/GenericShooter/Addons/Common/Blueprints/BaseClasses/BP_SlotInventory_ItemInfo_Base Object Reference"))
  (bind _returnvalue (`self.GetOwner`))
  (bind _iteminfos (`self.ItemInfos`))
  (bind _returnvalue_2 (`|SpawnActorFromClass` NewItemInfoClass (`KismetMathLibrary.MakeTransform` (0.0 0.0 0.0)) "AlwaysSpawn" "OverrideRootScale" _returnvalue (cast `Pawn` _returnvalue :!pure true)))
  (set `local.LocalNewItemInfo` _returnvalue_2)
  (if (`/Game/GenericShooter/Addons/Common/Blueprints/BaseClasses/BP_SlotInventory_ItemInfo_Base.CanBeAdded` (`local.LocalNewItemInfo`) (`self.GetOwner`) (`self.ItemInfos`))
    (`KismetArrayLibrary.Array_Add` _iteminfos (`local.LocalNewItemInfo`))
    (`self.SortItemsByPriority`)
    (bind _weaponbarwidget (`self.WeaponBarWidget`)
      (:`then`
        (set `/Game/GenericShooter/Addons/SlotInventory/Core/UI/WBP_SlotInventory.ItemReferences` _iteminfos _weaponbarwidget)
        (if (`local.bRebuildBar`)
          (`self.RebuildBar`)
          (return (`local.LocalNewItemInfo`) true)
          (else
            (return (`local.LocalNewItemInfo`) true))))
      (:`else`
        (return (`local.LocalNewItemInfo`) true)))
    (else
      (`Actor.K2_DestroyActor` (`local.LocalNewItemInfo`))
      (return null false))))

(fn `AttemptSwitchToSlot`
  (params (Slot :type Integer) (CurrentItem :type "/Game/GenericShooter/Addons/Common/Blueprints/BaseClasses/BP_SlotInventory_ItemInfo_Base Object Reference") (bBackwards :type Boolean))
  (locals (Items :type "Array of /Game/GenericShooter/Addons/Common/Blueprints/BaseClasses/BP_SlotInventory_ItemInfo_Base Object Reference") (CurrentlySelectedIndex :type Integer))
  (bind _returnvalue (`KismetArrayLibrary.Array_Find` (`local.Items`) (`self.SelectedItem`)))
  (bind _returnvalue_2 (`KismetArrayLibrary.Array_Length` (`local.Items`)))
  (bind _returnvalue_3 (mod (+ (+ _returnvalue (`KismetMathLibrary.SelectInt` -1 1 (`local.bBackwards`))) _returnvalue_2) _returnvalue_2))
  (`|ExecutionSequence`
    (:`then_0`
      ;[1 1 1] If initially trying to select, use our current item as our selected item.
      (if (and (`KismetSystemLibrary.IsValid` (`local.CurrentItem`)) (not (`KismetSystemLibrary.IsValid` (`self.SelectedItem`))))
        (set `self.SelectedItem` (`local.CurrentItem`))))
    (:`then_1`
      ;[1 1 1] If initially trying to select, use our gameplay active item as our selected item.
      (if (and (`KismetSystemLibrary.IsValid` (`self.GameplayActiveItem`)) (not (`KismetSystemLibrary.IsValid` (`self.SelectedItem`))))
        (set `self.SelectedItem` (`self.GameplayActiveItem`))))
    (:`then_2`
      (bind _items (`self.GetItemsInSlot` (`local.Slot`)))
      (set `local.Items` _items)
      (if (> (`KismetArrayLibrary.Array_Length` _items) 0)
        ;[1 1 1] Increment Slot Selection
        (if (!= _returnvalue -1)
          (bind _output_get (set `local.CurrentlySelectedIndex` _returnvalue))
          (if (!= _output_get _returnvalue_3)
            (set `self.SelectedItem` (`|GetArrayItem` (`local.Items`) _returnvalue_3)))
          (else
            (set `self.SelectedItem` (`|GetArrayItem` (`local.Items`)))))
        (else
          ;[1 1 1] Handle selecting an empty slot
          (if (`self.bIgnoreEmptySlotAttempts`)
            (return)
            (else
              (set `self.SelectedItem` null))))))
    (:`then_3`
      (if (`self.bFastSwitch`)
        (`self.CommitToSelected`)
        (else
          ;[1 1 1] If UI is present, tell it what we've selected
          (bind _weaponbarwidget (`self.WeaponBarWidget`)
            (:`then`
              _)
            (:`else`
              (`self.CreateWeaponBarWidget`)))
          (`self.WeaponBarWidget`
            (:`then`
              (`/Game/GenericShooter/Addons/SlotInventory/Core/UI/WBP_SlotInventory.SetSelectedItem` _weaponbarwidget (`self.SelectedItem`))
              (`/Game/GenericShooter/Addons/SlotInventory/Core/UI/WBP_SlotInventory.SetBarVisibility` (`self.WeaponBarWidget`) true))
            (:`else`)))))))

(fn `CanAddItem`
  (params (ItemInfo :type "/Game/GenericShooter/Addons/Common/Blueprints/BaseClasses/BP_SlotInventory_ItemInfo_Base Object Reference"))
  (returns (bCanAdd :type Boolean))
  (return (`/Game/GenericShooter/Addons/Common/Blueprints/BaseClasses/BP_SlotInventory_ItemInfo_Base.CanBeAdded` ItemInfo (`self.GetOwner`) (`self.ItemInfos`))))

(fn `Cleanup`
  (params (bClearItemInfoReferences :type Boolean))
  (`self.ClearWidget`)
  (set `self.SelectedItem` null)
  (set `self.GameplayActiveItem` null)
  (if (`local.bClearItemInfoReferences`)
    (`KismetArrayLibrary.Array_Clear` (`self.ItemInfos`))
    (return)
    (else
      (return))))

(fn `ClearWidget`
  (bind _weaponbarwidget (`self.WeaponBarWidget`)
    (:`then`
      (`Widget.RemoveFromParent` _weaponbarwidget)
      (set `self.WeaponBarWidget` null)
      (return))
    (:`else`
      (return))))

(fn `CommitToSelected`
  (returns (bShouldConsume :type Boolean))
  (bind _weaponbarwidget (`self.WeaponBarWidget`))
  (bind _selecteditem (`self.SelectedItem`)
    (:`then`
      (if (`KismetArrayLibrary.Array_Contains` (`self.ItemInfos`) _selecteditem)
        (`self.OnItemSelected` _selecteditem))
      (set `self.SelectedItem` null)
      (`/Engine/EditorBlueprintResources/StandardMacros.IsValid` _weaponbarwidget
        (:`Is Valid`
          (`/Game/GenericShooter/Addons/SlotInventory/Core/UI/WBP_SlotInventory.SetSelectedItem` _weaponbarwidget null)
          (`/Game/GenericShooter/Addons/SlotInventory/Core/UI/WBP_SlotInventory.SetBarVisibility` (`self.WeaponBarWidget`) (not (`self.bHideWhenNotSelecting`)))
          (return true))
        (:`Is Not Valid`
          (return true))))
    (:`else`
      (return false))))

(fn `CreateWeaponBarWidget`
  (bind _weaponbarwidget (`self.WeaponBarWidget`))
  (`self.WeaponBarWidget`
    (:`then`
      (return))
    (:`else`
      (bind _ascharacter (cast `Character` (`self.GetOwner`))
        (:`then`
          (if (`Pawn.IsLocallyControlled` _ascharacter)
            (bind _asplayer_controller (cast `PlayerController` (`Pawn.GetController` _ascharacter))
              (:`then`
                (bind _returnvalue (`|CreateWidget` "/Game/GenericShooter/Addons/SlotInventory/Core/UI/WBP_SlotInventory.WBP_SlotInventory_C" _asplayer_controller (`self.NumSlots`)))
                (bind _output_get (set `self.WeaponBarWidget` _returnvalue))
                (`UserWidget.AddToPlayerScreen` _output_get 0)
                (set `/Game/GenericShooter/Addons/SlotInventory/Core/UI/WBP_SlotInventory.ItemReferences` (`self.ItemInfos`) _weaponbarwidget)
                (`/Game/GenericShooter/Addons/SlotInventory/Core/UI/WBP_SlotInventory.BuildSlots` _weaponbarwidget)
                (`/Game/GenericShooter/Addons/SlotInventory/Core/UI/WBP_SlotInventory.SetBarVisibility` _weaponbarwidget (not (`self.bHideWhenNotSelecting`)))
                (`self.OnWidgetCreated` (`self.WeaponBarWidget`))
                (return))
              (:`CastFailed`
                _)))
          (return))
        (:`CastFailed`
          (return))))))

(fn `GetHighestPriorityItemInLowestSlot`
  (params (FilterClass :type "/Game/GenericShooter/Addons/Common/Blueprints/BaseClasses/BP_SlotInventory_ItemInfo_Base Class Reference"))
  (returns (ItemInfo :type "/Game/GenericShooter/Addons/Common/Blueprints/BaseClasses/BP_SlotInventory_ItemInfo_Base Object Reference"))
  (locals (bFilterClass :type Boolean))
  (if (> (`KismetArrayLibrary.Array_Length` (`self.ItemInfos`)) 0)
    (if (!= FilterClass null)
      (for _array_element (`self.ItemInfos`)
        (if (`KismetMathLibrary.ClassIsChildOf` (`GameplayStatics.GetObjectClass` _array_element) (`local.FilterClass`))
          (return _array_element)))
      (return null)
      (else
        (return (`|GetArrayItem` (`self.ItemInfos`)))))
    (else
      (return null))))

(fn `GetItemsInSlot`
  (params (Slot :type Integer))
  (returns (Items :type "Array of /Game/GenericShooter/Addons/Common/Blueprints/BaseClasses/BP_SlotInventory_ItemInfo_Base Object Reference") (Num :type Integer))
  (locals (ItemInfosInSlot :type "Array of /Game/GenericShooter/Addons/Common/Blueprints/BaseClasses/BP_SlotInventory_ItemInfo_Base Object Reference"))
  (bind _iteminfosinslot (`local.ItemInfosInSlot`))
  (for _array_element (`self.ItemInfos`)
    (if (== (`/Game/GenericShooter/Addons/Common/Blueprints/BaseClasses/BP_SlotInventory_ItemInfo_Base.Slot` _array_element) Slot)
      (`KismetArrayLibrary.Array_Add` (`local.ItemInfosInSlot`) _array_element)))
  (return _iteminfosinslot (`KismetArrayLibrary.Array_Length` _iteminfosinslot)))

(fn `GetItemsOfClass`
  (params (ItemInfoClass :type "/Game/GenericShooter/Addons/Common/Blueprints/BaseClasses/BP_SlotInventory_ItemInfo_Base Class Reference"))
  (returns (Items :type "Array of /Game/GenericShooter/Addons/Common/Blueprints/BaseClasses/BP_SlotInventory_ItemInfo_Base Object Reference") (Num :type Integer))
  (locals (OutItems :type "Array of /Game/GenericShooter/Addons/Common/Blueprints/BaseClasses/BP_SlotInventory_ItemInfo_Base Object Reference"))
  (bind _iteminfos (`self.ItemInfos`))
  (bind _outitems (`local.OutItems`))
  (if (`KismetSystemLibrary.IsValidClass` ItemInfoClass)
    (for _array_element (`self.ItemInfos`)
      (if (`KismetMathLibrary.ClassIsChildOf` (`GameplayStatics.GetObjectClass` _array_element) (`local.ItemInfoClass`))
        (`KismetArrayLibrary.Array_Add` (`local.OutItems`) _array_element)))
    (return _outitems (`KismetArrayLibrary.Array_Length` _outitems))
    (else
      (return _iteminfos (`KismetArrayLibrary.Array_Length` _iteminfos)))))

(fn `GetNextItemInSlot`
  (params (StartingItem :type "/Game/GenericShooter/Addons/Common/Blueprints/BaseClasses/BP_SlotInventory_ItemInfo_Base Object Reference") (bBackwards :type Boolean))
  (returns (Item :type "/Game/GenericShooter/Addons/Common/Blueprints/BaseClasses/BP_SlotInventory_ItemInfo_Base Object Reference"))
  (locals (SlotItems :type Boolean))
  (`/Engine/EditorBlueprintResources/StandardMacros.IsValid` StartingItem
    (:`Is Valid`
      (bind (_items _num) (`self.GetItemsInSlot` (`/Game/GenericShooter/Addons/Common/Blueprints/BaseClasses/BP_SlotInventory_ItemInfo_Base.Slot` (`local.StartingItem`))))
      (if (<= _num 1)
        (return (`|GetArrayItem` _items (mod (+ (`KismetArrayLibrary.Array_Find` _items (`local.StartingItem`)) _num (`KismetMathLibrary.SelectInt` -1 1 (`local.bBackwards`))) _num)))
        (else
          (return null))))
    (:`Is Not Valid`
      (return null))))

(fn `OnRep_ItemInfos`
  (bind _weaponbarwidget (`self.WeaponBarWidget`)
    (:`then`
      (set `/Game/GenericShooter/Addons/SlotInventory/Core/UI/WBP_SlotInventory.ItemReferences` (`self.ItemInfos`) _weaponbarwidget)
      (`/Game/GenericShooter/Addons/SlotInventory/Core/UI/WBP_SlotInventory.BuildSlots` _weaponbarwidget)
      (return))
    (:`else`
      (return))))

(fn `RebuildBar`
  (bind _weaponbarwidget (`self.WeaponBarWidget`)
    (:`then`
      (`/Game/GenericShooter/Addons/SlotInventory/Core/UI/WBP_SlotInventory.BuildSlots` _weaponbarwidget)
      (bind _selecteditem (`self.SelectedItem`)
        (:`then`
          (`/Game/GenericShooter/Addons/SlotInventory/Core/UI/WBP_SlotInventory.SetSelectedItem` _weaponbarwidget null)
          (`/Game/GenericShooter/Addons/SlotInventory/Core/UI/WBP_SlotInventory.SetSelectedItem` _weaponbarwidget _selecteditem)
          (return))
        (:`else`
          (return))))
    (:`else`
      (return))))

(fn `RemoveItem`
  (params (ItemToRemove :type "/Game/GenericShooter/Addons/Common/Blueprints/BaseClasses/BP_SlotInventory_ItemInfo_Base Object Reference") (bSkipSelectingAnotherIfItemWasSelected :type Boolean))
  (returns (bRemoved :type Boolean))
  (locals (bWasRemoved :type Boolean) (NextItem :type Boolean))
  (bind _weaponbarwidget (`self.WeaponBarWidget`))
  (`|ExecutionSequence`
    (:`then_0`
      ;[1 1 1] If item being removed wasn't selected, simply remove it and continue
      (if (== (`self.SelectedItem`) (`local.ItemToRemove`))
        (if (`KismetArrayLibrary.Array_Contains` (`self.ItemInfos`) (`local.ItemToRemove`))
          ;[1 1 1] If removing selected item attempt to switch to another item in our inventory. First we try to switch to the next item in the removing item's slot, otherwise we switch to highest priority item.
          (if (not (`local.bSkipSelectingAnotherIfItemWasSelected`))
            (bind _item (`self.GetNextItemInSlot` (`local.ItemToRemove`)))
            (`/Engine/EditorBlueprintResources/StandardMacros.IsValid` _item
              (:`Is Valid`
                (set `self.SelectedItem` _item))
              (:`Is Not Valid`
                (set `self.SelectedItem` (`self.GetHighestPriorityItemInLowestSlot` null))))
            (else
              (set `self.SelectedItem` null)))
          (bind _returnvalue (`KismetArrayLibrary.Array_RemoveItem` (`self.ItemInfos`) (`local.ItemToRemove`)))
          (bind _output_get (set `local.bWasRemoved` _returnvalue))
          (if _output_get
            (`self.OnSelectedItemRemoved` (`local.ItemToRemove`))))
        (else
          (bind _returnvalue_2 (`KismetArrayLibrary.Array_RemoveItem` (`self.ItemInfos`) (`local.ItemToRemove`)))
          (set `local.bWasRemoved` _returnvalue_2))))
    (:`then_1`
      ;[1 1 1] If we removed the gameplay active item, notify anyone who needs to know
      (if (and (== (`self.GameplayActiveItem`) (`local.ItemToRemove`)) (`local.bWasRemoved`))
        (set `self.GameplayActiveItem` null)
        (`self.OnGameplayActiveItemRemoved` (`local.ItemToRemove`))))
    (:`then_2`
      ;[1 1 1] If item wasn't removed, do nothing
      (if (`local.bWasRemoved`)
        ;[1 1 1] Update UI, then finally call OnItemRemoved
        (`|ExecutionSequence`
          (:`then_0`
            (`/Engine/EditorBlueprintResources/StandardMacros.IsValid` _weaponbarwidget
              (:`Is Valid`
                (`KismetArrayLibrary.Array_RemoveItem` (`/Game/GenericShooter/Addons/SlotInventory/Core/UI/WBP_SlotInventory.ItemReferences` _weaponbarwidget) (`local.ItemToRemove`))
                (`self.RebuildBar`))))
          (:`then_1`
            (`self.OnItemRemoved` (`local.ItemToRemove`))
            (return true))
          (:`then_2`
            (`self.SelectedItem`
              (:`then`
                (if (`self.bFastSwitch`)
                  (`self.CommitToSelected`)))
              (:`else`))))
        (else
          (return true))))))

(fn `RemoveItemsOfClass`
  (params (ItemClass :type "/Game/GenericShooter/Addons/Common/Blueprints/BaseClasses/BP_SlotInventory_ItemInfo_Base Class Reference"))
  (returns (NumRemoved :type Integer))
  (locals (RemoveCount :type Integer))
  (bind _items (`self.GetItemsOfClass` ItemClass))
  (for _array_element _items
    (`self.RemoveItem` _array_element)
    (`/Engine/EditorBlueprintResources/StandardMacros.IncrementInt` (`local.RemoveCount`)))
  (return (`local.RemoveCount`)))

(fn `SortItemsByPriority`
  (locals (SortedItems :type "Array of /Game/GenericShooter/Addons/Common/Blueprints/BaseClasses/BP_SlotInventory_ItemInfo_Base Object Reference") (bAdded :type Boolean))
  (if (> (`KismetArrayLibrary.Array_Length` (`self.ItemInfos`)) 1)
    (`KismetArrayLibrary.Array_Add` (`local.SortedItems`) (`|GetArrayItem` (`self.ItemInfos`)))
    (for _index (range 1 (+ (`KismetArrayLibrary.Array_LastIndex` (`self.ItemInfos`)) 1))
      (set `local.bAdded` false)
      (for (_array_element _array_index) (`local.SortedItems`)
        (bind _output (`|GetArrayItem` (`self.ItemInfos`) _index))
        (if (`/Game/GenericShooter/Addons/Common/Blueprints/BaseClasses/BP_SlotInventory_ItemInfo_Base.IsHigherPriorityThan` _output _array_element)
          (`KismetArrayLibrary.Array_Insert` (`local.SortedItems`) _output _array_index)
          (set `local.bAdded` true)
          (break)))
      (if (not (`local.bAdded`))
        (`KismetArrayLibrary.Array_Add` (`local.SortedItems`) _output)))
    (set `self.ItemInfos` (`local.SortedItems`))
    (return)
    (else
      (return))))