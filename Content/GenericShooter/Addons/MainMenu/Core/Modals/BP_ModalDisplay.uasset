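; Manages the main menu addon's stack of modal popup widgets, including error popups for network and travel failures.
; CreateModalPopup builds each widget under the game instance owner and tracks it in Modals, using a count-based Z-order to layer newer ones on top.
; Modals close by ID through simulated button presses, and DestroyModal restores keyboard focus.
; Failure enums map to a stored error text, which CreateErrorModalIfNeeded later displays and clears.
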(fn `ClearLastError`
  (set `self.LastErrorText` "")
  (return))

(fn `CloseModalsWithID`
  (params (ModalID :type Name) (ButtonIDToPress :type Integer))
  ;[1 1 1] Loop through all active modals, then return
  (for _array_element (`self.Modals`)
    ;[1 1 1] If an active modal with the searched for ID is found, close it by hitting the desired button
    (if (== (`/Game/GenericShooter/Addons/MainMenu/Core/Modals/WBP_ModalPopup.ID` _array_element) ModalID)
      (`/Game/GenericShooter/Addons/MainMenu/Core/Modals/WBP_ModalPopup.SimulateButtonPress` _array_element (`local.ButtonIDToPress`))))
  (return))

(fn `CreateErrorModalIfNeeded`
  (params (PlayerController :type "PlayerController Object Reference") (WidgetToFocusOnClose :type "UserWidget Object Reference"))
  (if (`KismetTextLibrary.TextIsEmpty` (`self.LastErrorText`))
    (return)
    (else
      (`self.CreateModalPopup` PlayerController "Error" (`self.LastErrorText`) (`|MakeArray` "OK" :!type "Text") false true 0.0 0 WidgetToFocusOnClose)
      (`self.ClearLastError`)
      (return))))

(fn `CreateModalPopup`
  (params (TargetPlayerController :type "PlayerController Object Reference (by ref)") (ModalID :type Name) (Title :type Text) (ButtonLabels :type "Array of Text") (bIsThrobbingWidget :type Boolean) (bCloseOnAnyButtonPress :type Boolean :default true) (ExpireTime :type "Float (double-precision)") (ButtonIdToFireOnExpiration :type Integer) (WidgetToFocusOnClose :type "UserWidget Object Reference"))
  (returns (Modal :type "/Game/GenericShooter/Addons/MainMenu/Core/Modals/WBP_ModalPopup Object Reference"))
  (bind _returnvalue (`|GenericCreateObject` (`self.ModalWidgetClass`) (`self.GameInstanceOwner`) Title ModalID bIsThrobbingWidget ButtonLabels ExpireTime ButtonIdToFireOnExpiration bCloseOnAnyButtonPress self WidgetToFocusOnClose))
  (`UserWidget.SetOwningPlayer` _returnvalue (`local.TargetPlayerController`))
  ;[1 1 1] Add to our list of active Modals
  (`KismetArrayLibrary.Array_Add` (`self.Modals`) _returnvalue)
  ;[1 1 1] Add Modal widget to the screen
  (`UserWidget.AddToViewport` _returnvalue (+ (`KismetArrayLibrary.Array_Length` (`self.Modals`)) 1000))
  (return _returnvalue))

(fn `DestroyAllModals`
  (bind _modals (`self.Modals`))
  ;[1 1 1] Loop through all Modals, then clear the Modal stack
  (for _array_element _modals
    ;[1 1 1] If a modal is valid, remove it from the parent
    (`/Engine/EditorBlueprintResources/StandardMacros.IsValid` _array_element
      (:`Is Valid`
        (`Widget.RemoveFromParent` _array_element))))
  (`KismetArrayLibrary.Array_Clear` _modals)
  (return))

(fn `DestroyModal`
  (params (Modal :type "/Game/GenericShooter/Addons/MainMenu/Core/Modals/WBP_ModalPopup Object Reference") (bSkipRemoveFromParent :type Boolean))
  ;[1 1 1] Remove Modal from active Modals
  (`KismetArrayLibrary.Array_RemoveItem` (`self.Modals`) Modal)
  ;[1 1 1] If we need to set focus on close, do so
  (bind _widgettofocusonclose (`/Game/GenericShooter/Addons/MainMenu/Core/Modals/WBP_ModalPopup.WidgetToFocusOnClose` (`local.Modal`))
    (:`then`
      (`Widget.SetKeyboardFocus` _widgettofocusonclose))
    (:`else`
      _))
  ;[1 1 1] If removing from parent isn't skipped, remove
  (if (`local.bSkipRemoveFromParent`)
    (return)
    (else
      (`Widget.RemoveFromParent` (`local.Modal`))
      (return))))

(fn `GetModalByID`
  (params (ModalID :type Name))
  (returns (Result :type "/Game/GenericShooter/Addons/MainMenu/Core/Modals/WBP_ModalPopup Object Reference"))
  ;[1 1 1] Loop through all active Modals
  (for _array_element (`self.Modals`)
    ;[1 1 1] If we find a match, return it...
    (if (== (`local.ModalID`) (`/Game/GenericShooter/Addons/MainMenu/Core/Modals/WBP_ModalPopup.ID` _array_element))
      (return _array_element)))
  ;[1 1 1] ...otherwise return nothing
  (return null))

(fn `SetErrorFromNetworkError`
  (params (NetworkError :type "ENetworkFailure Enum" :default "NetDriverAlreadyExists"))
  (`self.SetLastErrorText` (select `ENetworkFailure` NetworkError :`NetDriverAlreadyExists` "Network Error: Net Driver Already Exists" :`NetDriverCreateFailure` "Network Error: Failed to create Net Driver" :`NetDriverListenFailure` "Network Error: Net Driver failed to Listen" :`ConnectionLost` "Network Error: Lost Connection to Host" :`ConnectionTimeout` "Network Error: Connection Timed Out" :`FailureReceived` "Network Error: Failure Received" :`OutdatedClient` "Network Error: Client is out of date. Try updating?" :`OutdatedServer` "Network Error: Server is out of date" :`PendingConnectionFailure` "Network Error: Failed to Connect" :`NetGuidMismatch` "Network Error: Net Guid Mismatch" :`NetChecksumMismatch` "Network Error: Net Checksum Mismatch" :!type "Text"))
  (return))

(fn `SetErrorFromTravelFailure`
  (params (TravelFailure :type "ETravelFailure Enum" :default "NoLevel"))
  (`self.SetLastErrorText` (select `ETravelFailure` TravelFailure :`NoLevel` "Travel Error: No Level" :`LoadMapFailure` "Travel Error: Failed to Load Map" :`InvalidURL` "Travel Error: Invalid URL" :`PackageMissing` "Travel Error: Package Missing" :`PackageVersion` "Travel Error: Bad Package Version" :`NoDownload` "Travel Error: No Download" :`TravelFailure` "Travel Error: Failed to Travel (Reason: Unknown)" :`CheatCommands` "Travel Error: Cheat Commands?" :`PendingNetGameCreateFailure` "Travel Error: Failed to Create Net Game" :`CloudSaveFailure` "Travel Error: Failed to Save to Cloud" :`ServerTravelFailure` "Travel Error: Server Travel Failed" :`ClientTravelFailure` "Travel Error: Client Travel Failed" :!type "Text"))
  (return))

(fn `SetLastErrorText`
  (params (ErrorText :type Text))
  (set `self.LastErrorText` ErrorText)
  (return))