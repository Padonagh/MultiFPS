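; Main menu option that offers an integer range as a list of selectable choices.
; BuildValues fills Choices by stepping from Min to Max by Step, tagging each entry with its number and selecting the one that equals DefaultValue.
; CreateWidget builds these values before calling the parent implementation, and GetOptionValueAsInteger converts the option's string value back to an integer.
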(fn `BuildValues`
  (returns (bBuiltValues :type Boolean))
  (locals (CurrentValue :type Integer))
  (bind _currentvalue (`local.CurrentValue`))
  (`KismetArrayLibrary.Array_Clear` (`self.Choices`))
  (set `local.CurrentValue` (`self.Min`))
  (while (and (>= (`local.CurrentValue`) (`self.Min`)) (<= (`local.CurrentValue`) (`self.Max`)) (!= (`self.Step`) 0))
    (`|ExecutionSequence`
      (:`then_0`
        ;[1 1 1] Add integer to choice, if default value, set our selected choice to this choice
        (bind _returnvalue (`KismetArrayLibrary.Array_Add` (`self.Choices`) (make `/Game/GenericShooter/Addons/MainMenu/Core/Controls/FTaggedText` (`KismetTextLibrary.Conv_IntToText` _currentvalue) (`KismetStringLibrary.Conv_IntToString` _currentvalue))))
        (if (== (`local.CurrentValue`) (`self.DefaultValue`))
          (set `self.SelectedChoice` _returnvalue)))
      (:`then_1`
        ;[1 1 1] Increment by step
        (set `local.CurrentValue` (+ (`local.CurrentValue`) (`self.Step`))))))
  (return true))

(fn `CreateWidget`
  (params (OwningPlayerController :type "PlayerController Object Reference") (GameInstance :type "GameInstance Object Reference"))
  (returns (OptionWidget :type "UserWidget Object Reference"))
  (`self.BuildValues`)
  (bind _optionwidget (`parent.CreateWidget` OwningPlayerController GameInstance))
  (return _optionwidget))

(fn `GetOptionValueAsInteger`
  (returns (Value :type Integer))
  (bind _value (`self.GetOptionValueAsString`))
  (return (`KismetStringLibrary.Conv_StringToInt` _value)))