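; Death camera actor that smoothly rotates to track a dead actor while it serves as a view target.
; Tick starts when it becomes the view target, stops if the dead actor is invalid, and the camera destroys itself when it stops being viewed.
; LookAtTarget interpolates rotation toward a named bone or socket on the dead component, falling back to the component or actor location.
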(event `self.K2_OnBecomeViewTarget`
  (params (PC :type "PlayerController Object Reference"))
  (`self.SetActorTickEnabled` true))

(event `self.ReceiveBeginPlay`
  (`self.DeadActor`
    (:`then`
      (bind _deadcomponent (`self.DeadComponent`)
        (:`then`
          (set `self.bUseSocket` (`SceneComponent.DoesSocketExist` _deadcomponent (`self.DeadBoneOrSocketName`))))
        (:`else`)))
    (:`else`
      (`self.SetActorTickEnabled` false))))

(event `self.ReceiveTick`
  (params (DeltaSeconds :type "Float (single-precision)"))
  (`self.DeadActor`
    (:`then`
      (`self.LookAtTarget` DeltaSeconds))
    (:`else`
      (`self.SetActorTickEnabled` false))))

(event `self.K2_OnEndViewTarget`
  (params (PC :type "PlayerController Object Reference"))
  (`self.K2_DestroyActor`))

(fn `LookAtTarget`
  (params (DeltaSeconds :type "Float (double-precision)"))
  (locals (TargetLocation :type "Vector Structure"))
  (`|ExecutionSequence`
    (:`then_0`
      ;[1 1 1] Attempt to get component socket as tracking location, if not, fall back to what we can reliably track
      (`self.DeadComponent`
        (:`then`
          (if (`self.bUseSocket`)
            (set `local.TargetLocation` (`SceneComponent.GetSocketLocation` (`self.DeadComponent`) (`self.DeadBoneOrSocketName`)))
            (else
              (set `local.TargetLocation` (`SceneComponent.K2_GetComponentLocation` (`self.DeadComponent`))))))
        (:`else`
          (set `local.TargetLocation` (`self.K2_GetActorLocation` (`self.DeadActor`))))))
    (:`then_1`
      ;[1 1 1] Update camera rotation
      (`self.K2_SetActorRotation` (`KismetMathLibrary.RInterpTo` (`self.K2_GetActorRotation`) (`KismetMathLibrary.FindLookAtRotation` (`self.K2_GetActorLocation`) (`local.TargetLocation`)) (`local.DeltaSeconds`) (`self.TrackingSpeed`)) true)
      (return))))

(fn `UserConstructionScript`)