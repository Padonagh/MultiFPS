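; Character component that manages tagged cameras, tracks the replicated active camera by name and reports its view with optional weapon FOV override.
; On BeginPlay it indexes owner cameras and components by tag, then toggles first- and third-person visibility from camera and local control.
; Camera changes go through a server RPC, while Tick aligns first-person components to the eyes viewpoint.
; On death it spawns a tracking camera from randomly picked eligible cameras and blends to it.
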(event `self.ReceiveBeginPlay`
  (`KismetSystemLibrary.Delay` 0.0) ; Takes 1 frame to update locally controlled status
  (`self.BuildCameraList`)
  (`self.GetManagedComponents`)
  (`self.SetActiveCamera` (`self.ActiveCamera`)))

(event `self.ReceiveTick`
  (params (DeltaSeconds :type "Float (single-precision)"))
  (`self.SyncFirstPersonComponents`))

(event `ServerSetActiveCamera`
  (params (CameraName :type Name))
  (`self.SetActiveCamera` CameraName))

(fn `BuildCameraList`
  (locals (TestCameraComponent :type "CameraComponent Object Reference"))
  (bind _componenttags (`ActorComponent.ComponentTags` (`local.TestCameraComponent`)))
  (bind _output (`|GetArrayItem` _componenttags))
  (for _array_element (`Actor.K2_GetComponentsByClass` (`self.GetOwner`) "/Script/Engine.CameraComponent")
    (set `local.TestCameraComponent` _array_element)
    (`|ExecutionSequence`
      (:`then_0`
        ;[1 1 1] Builds primary camera list
        (if (`KismetArrayLibrary.Array_IsValidIndex` _componenttags)
          (if (`.ReturnValue` (`BlueprintMapLibrary.Map_Find` (`self.Cameras`) _output))
            (`KismetSystemLibrary.PrintString` "BP_CharacterCameraManagerComponent can not distinguish between character camera types. Multiple cameras have the same first component tag." true true (struct :`R` 1.0 :`G` 0.07603 :`A` 1.0) 10.0)
            (else
              (`BlueprintMapLibrary.Map_Add` (`self.Cameras`) _output (`local.TestCameraComponent`))))
          (else
            (`KismetSystemLibrary.PrintString` "BP_CharacterCameraManagerComponent can not determine purpose for found camera. Make sure every camera in character has a component tag assigned." true true (struct :`R` 1.0 :`G` 0.07603 :`A` 1.0) 10.0))))
      (:`then_1`
        ;[1 1 1] Builds death elegible camera list
        (if (!= (`KismetArrayLibrary.Array_Find` (`ActorComponent.ComponentTags` (`local.TestCameraComponent`)) (`self.DeathEligibleCameraTag`)) -1)
          (`BlueprintSetLibrary.Set_Add` (`self.DeathElegibleCameras`) (`local.TestCameraComponent`))))))
  (return))

(fn `CreateAndTargetDeathCameraActor`
  (returns (DeathCamera :type "CameraActor Object Reference"))
  (locals (LocalController :type "PlayerController Object Reference"))
  (bind _localpc (`self.GetControlledPC`))
  (bind _returnvalue (`self.GetOwner`))
  (bind _aspawn (cast `Pawn` _returnvalue :!pure true))
  (`/Engine/EditorBlueprintResources/StandardMacros.IsValid` _localpc
    (:`Is Valid`
      (set `local.LocalController` _localpc))
    (:`Is Not Valid`
      (set `local.LocalController` (`self.LastKnownLocalPlayerController`))))
  (`local.LocalController`
    (:`then`
      (if (== (`BlueprintSetLibrary.Set_Length` (`self.DeathElegibleCameras`)) 0)
        (`KismetSystemLibrary.PrintString` "ERROR: BP_CharacerCameraManagerComponent was told to create and target death camera but has no eligible death cameras!" true true (struct :`R` 1.0 :`G` 0.025124 :`A` 1.0) 10.0)
        (return null)
        (else
          ;[1 1 1] Get random eligible death camera and spawn a camera actor at its location
          (bind _result (`BlueprintSetLibrary.Set_ToArray` (`self.DeathElegibleCameras`)))
          (bind _output (`|GetArrayItem` _result (`KismetMathLibrary.RandomIntegerInRange` 0 (- (`BlueprintSetLibrary.Set_Length` (`self.DeathElegibleCameras`)) 1))))
          (bind _returnvalue_2 (`|SpawnActorFromClass` "/Game/GenericShooter/Addons/CharacterCameraManager/Core/BP_CharacterDeathCamera.BP_CharacterDeathCamera_C" (`KismetMathLibrary.MakeTransform` (`SceneComponent.K2_GetComponentLocation` _output) (`SceneComponent.K2_GetComponentRotation` _output)) "AdjustIfPossibleButAlwaysSpawn" "OverrideRootScale" (`Pawn.GetController` _aspawn) _returnvalue (`self.DeathTrackingComponent`) (`self.DeathCameraTrackingSocketBoneName`) _aspawn))
          (set `Actor.Tags` (`|MakeArray` (`self.DeathEligibleCameraTag`)) _returnvalue_2)
          (set `self.ActiveCamera` (`self.DeathTrackingComponentTag`))
          (`PlayerController.SetViewTargetWithBlend` (`local.LocalController`) _returnvalue_2 0.25 "VTBlend_Linear" 0.0 true)
          (`self.OnActiveCameraChanged` (`self.GetActiveCameraName`))
          (return _returnvalue_2))))
    (:`else`
      (return null))))

(fn `GetActiveCameraComponent`
  (returns (ActiveCameraComponent :type "CameraComponent Object Reference"))
  (bind (_value _returnvalue) (`BlueprintMapLibrary.Map_Find` (`self.Cameras`) (`self.ActiveCamera`)))
  (if _returnvalue
    (return _value)
    (else
      (return null))))

(fn `GetActiveCameraInfo`
  (returns (Location :type "Vector Structure") (Rotation :type "Rotator Structure") (FOV :type "Float (double-precision)"))
  (bind _activecameracomponent (`self.GetActiveCameraComponent`))
  (bind _weapondesiredfov (`self.WeaponDesiredFOV`))
  (bind _weapondesiredfov_2 (`self.WeaponDesiredFOV`))
  (bind _weapondesiredfov_3 (`self.WeaponDesiredFOV`))
  (bind (_outlocation _outrotation) (`Actor.GetActorEyesViewPoint` (`self.GetOwner`)))
  (if (== (`self.ActiveCamera`) (`self.ActorEyesViewPointCameraName`))
    (return _outlocation _outrotation (`KismetMathLibrary.SelectFloat` _weapondesiredfov_2 (`self.DefaultFOV`) (!= _weapondesiredfov_2 0.0)))
    (else
      (`/Engine/EditorBlueprintResources/StandardMacros.IsValid` _activecameracomponent
        (:`Is Valid`
          (bind _desiredview (`CameraComponent.GetCameraView` _activecameracomponent 0.0))
          (bind (_location _rotation _fov) (break `MinimalViewInfo` _desiredview))
          (return _location _rotation (`KismetMathLibrary.SelectFloat` _weapondesiredfov_3 _fov (!= _weapondesiredfov_3 0.0))))
        (:`Is Not Valid`
          (`KismetSystemLibrary.PrintString` "ERROR: BP_PlayerCameraManagerComponent failed to get any meaningful camera info for the active camera mode.")
          (return (0.0 0.0 0.0) (struct) (`KismetMathLibrary.SelectFloat` _weapondesiredfov (`self.DefaultFOV`) (!= _weapondesiredfov 0.0))))))))

(fn `GetActiveCameraName`
  (returns (ActiveCameraName :type Name))
  (return (`self.ActiveCamera`)))

(fn `GetControlledPC`
  (returns (LocalPC :type "PlayerController Object Reference"))
  (bind _aspawn (cast `Pawn` (`self.GetOwner`))
    (:`then`
      (bind _asplayer_controller (cast `PlayerController` (`Pawn.GetController` _aspawn))
        (:`then`
          (return _asplayer_controller))
        (:`CastFailed`
          _)))
    (:`CastFailed`
      _))
  (return null))

(fn `GetManagedComponents`
  (locals (Component :type "SceneComponent Object Reference"))
  (`BlueprintSetLibrary.Set_Clear` (`self.ThirdPersonVisibleOnlyComponents`))
  (`BlueprintSetLibrary.Set_Clear` (`self.FirstPersonVisibleOnlyComponents`))
  (for _array_element (`Actor.K2_GetComponentsByClass` (`self.GetOwner`) "/Script/Engine.SceneComponent")
    (bind _output_get (set `local.Component` _array_element))
    (for _array_element_2 (`ActorComponent.ComponentTags` _output_get)
      (`|ExecutionSequence`
        (:`then_0`
          (if (`BlueprintSetLibrary.Set_Contains` (`self.ThirdPersonVisibleOnlyComponentTags`) _array_element_2)
            (`BlueprintSetLibrary.Set_Add` (`self.ThirdPersonVisibleOnlyComponents`) (`local.Component`))
            (elif (`BlueprintSetLibrary.Set_Contains` (`self.FirstPersonVisibleOnlyComponentTags`) _array_element_2)
              (`BlueprintSetLibrary.Set_Add` (`self.FirstPersonVisibleOnlyComponents`) (`local.Component`))
              (elif (`BlueprintSetLibrary.Set_Contains` (`self.FirstPersonComponentTagsToSyncWithActorEyesViewPoint`) _array_element_2)
                (`BlueprintSetLibrary.Set_Add` (`self.FirstPersonComponentsToSyncWithActorEyesViewPoint`) (`local.Component`))))))
        (:`then_1`
          ;[1 1 1] Find component to track on death
          (if (== _array_element_2 (`self.DeathTrackingComponentTag`))
            (set `self.DeathTrackingComponent` (`local.Component`)))))))
  (set `self.LastKnownLocalPlayerController` (`self.GetControlledPC`))
  (return))

(fn `IsInThirdPerson`
  (returns (bThirdPerson :type Boolean))
  (return (or (not (`BlueprintSetLibrary.Set_Contains` (`self.NotThirdPersonCameraNames`) (`self.ActiveCamera`))) (== (`self.ActiveCamera`) (`self.DeathEligibleCameraTag`)))))

(fn `OnRep_ActiveCamera`
  (`self.UpdateComponentVisibilities`)
  (`self.OnActiveCameraChanged` (`self.ActiveCamera`))
  (set `self.LastKnownLocalPlayerController` (`self.GetControlledPC`))
  (return))

(fn `SetActiveCamera`
  (params (CameraName :type Name))
  (if (not (`KismetSystemLibrary.IsServer`))
    (`self.ServerSetActiveCamera` CameraName))
  (set `self.ActiveCamera` CameraName)
  (`self.UpdateComponentVisibilities`)
  (return))

(fn `SetWeaponDesiredFOV`
  (params (NewFOV :type "Float (double-precision)"))
  (returns (bSet :type Boolean))
  (set `self.WeaponDesiredFOV` NewFOV)
  (return true))

(fn `SyncFirstPersonComponents`
  (bind _bupdatefirstpersoncomponentstosynconlyiflocallycontrolled (`self.bUpdateFirstPersonComponentsToSyncOnlyIfLocallyControlled`))
  (bind (_outlocation _outrotation) (`Actor.GetActorEyesViewPoint` (`self.GetOwner`)))
  (if (or (not _bupdatefirstpersoncomponentstosynconlyiflocallycontrolled) (and _bupdatefirstpersoncomponentstosynconlyiflocallycontrolled (`Pawn.IsLocallyControlled` (cast `Pawn` (`self.GetOwner`) :!pure true))))
    (bind _result (`BlueprintSetLibrary.Set_ToArray` (`self.FirstPersonComponentsToSyncWithActorEyesViewPoint`))) ; This however does not crash
    (`SceneComponent.K2_SetWorldLocationAndRotation` _result _outlocation _outrotation false false)
    (return)
    (else
      (return))))

(fn `UpdateComponentVisibilities`
  (bind _returnvalue (or (`self.IsInThirdPerson`) (and (not (`Pawn.IsLocallyControlled` (cast `Pawn` (`self.GetOwner`) :!pure true))) (`self.bForceThirdPersonVisibilityIfNotLocallyControlled`))))
  (bind _result (`BlueprintSetLibrary.Set_ToArray` (`self.FirstPersonVisibleOnlyComponents`)))
  (`SceneComponent.SetVisibility` _result (not _returnvalue) true)
  (bind _result_2 (`BlueprintSetLibrary.Set_ToArray` (`self.ThirdPersonVisibleOnlyComponents`)))
  (`SceneComponent.SetVisibility` _result_2 _returnvalue true)
  (return))