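; Actor component in the weapon system that stores the owner's ammo reserves per ammo type, each with current, max and infinite settings.
; Add, consume, set and query functions look up the type's array entry; adding respects the max and returns overflow, while consuming returns the shortfall.
; Only SetAmmo creates missing entries; add and consume print an error instead.
; Changes, including the AmmoStorage RepNotify, fire OnAmmoChanged.
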(fn `AddAmmo`
  (params (AmmoType :type "/Game/GenericShooter/Addons/WeaponSystem/Core/EWeaponAmmoType Enum" :default "NewEnumerator3") (AmmoDelta :type Integer) (bOverrideMaxAmmo :type Boolean))
  (returns (AmmoAdded :type Integer) (AmmoOverflow :type Integer))
  (locals (MaxFinalAmmoDelta :type Integer))
  ;[1 1 1] Make sure we're not adding negative ammo
  (if (> AmmoDelta 0)
    ;[1 1 1] Make sure ammo info type is defined.
    (bind (_ammoinfo _ammoindex _bhasammoinfo) (`self.GetAmmoInfoForAmmoType` (`local.AmmoType`)))
    (if _bhasammoinfo
      (bind _output (`|GetArrayItem` (`self.AmmoStorage`) _ammoindex))
      (bind (_ammotype _currentammo _maxammo) (break `/Game/GenericShooter/Addons/WeaponSystem/Core/FWeaponAmmoStorage` _output))
      ;[1 1 1] Grab ammo info, add delta to current ammo, return overflow.
      (bind _output_get (set `local.MaxFinalAmmoDelta` (`KismetMathLibrary.SelectInt` (`local.AmmoDelta`) (`KismetMathLibrary.Min` (- _maxammo _currentammo) (`local.AmmoDelta`)) (or (`local.bOverrideMaxAmmo`) (== _maxammo 0)))))
      (setmembers `/Game/GenericShooter/Addons/WeaponSystem/Core/FWeaponAmmoStorage` :`StructRef` _output :`CurrentAmmo` (+ _currentammo _output_get))
      (`self.OnAmmoChanged`)
      (return (`local.MaxFinalAmmoDelta`) (- (`local.AmmoDelta`) (`local.MaxFinalAmmoDelta`)))
      (else
        (`KismetSystemLibrary.PrintText` (`|FormatText` "{Parent}: {Me} tried adding {Amount} ammo for type {Type} but LooseAmmo does not have an element that defines ammo for {Type}." (`KismetTextLibrary.Conv_StringToText` (`KismetSystemLibrary.GetObjectName` (`self.GetOwner`))) (`KismetTextLibrary.Conv_StringToText` (`KismetSystemLibrary.GetObjectName` self)) (`local.AmmoDelta`) (`KismetTextLibrary.Conv_StringToText` (`KismetStringLibrary.Conv_ByteToString` (`local.AmmoType`)))))
        (return 0 (`local.AmmoDelta`))))
    (else
      (`KismetSystemLibrary.PrintText` (`|FormatText` "{Parent}: {Me} tried adding a negative amount of ammo ({Amount}) for type {Type}. Please use ConsumeAmmo instead." (`KismetTextLibrary.Conv_StringToText` (`KismetSystemLibrary.GetObjectName` (`self.GetOwner`))) (`KismetTextLibrary.Conv_StringToText` (`KismetSystemLibrary.GetObjectName` self)) (`local.AmmoDelta`) (`KismetTextLibrary.Conv_StringToText` (`KismetStringLibrary.Conv_ByteToString` (`local.AmmoType`)))))
      (return 0 (`local.AmmoDelta`)))))

(fn `CanHoldMoreAmmo`
  (params (AmmoType :type "/Game/GenericShooter/Addons/WeaponSystem/Core/EWeaponAmmoType Enum" :default "NewEnumerator3") (AmmoAmount :type Integer))
  (returns (bCanHoldMoreAmmo :type Boolean) (bCanHoldAllAmmo :type Boolean) (CanHoldAmount :type Integer))
  (bind (_ammoinfo _ammoindex _bhasammoinfo) (`self.GetAmmoInfoForAmmoType` AmmoType))
  (if _bhasammoinfo
    (bind (_ammotype _currentammo _maxammo) (break `/Game/GenericShooter/Addons/WeaponSystem/Core/FWeaponAmmoStorage` _ammoinfo))
    (bind _returnvalue (`KismetMathLibrary.Min` (- _maxammo _currentammo) AmmoAmount))
    (return (> _returnvalue 0) (>= _returnvalue AmmoAmount) _returnvalue)
    (else
      (return false false 0))))

(fn `ConsumeAmmo`
  (params (AmmoType :type "/Game/GenericShooter/Addons/WeaponSystem/Core/EWeaponAmmoType Enum" :default "NewEnumerator3") (AmmoDelta :type Integer))
  (returns (AmmoUnderflow :type Integer))
  (locals (FinalAmmoDelta :type Integer))
  (bind _ammodelta (`local.AmmoDelta`))
  ;[1 1 1] Make sure we're not consuming negative ammo
  (if (> AmmoDelta 0)
    ;[1 1 1] Make sure ammo info type is defined.
    (bind (_ammoinfo _ammoindex _bhasammoinfo) (`self.GetAmmoInfoForAmmoType` (`local.AmmoType`)))
    (if _bhasammoinfo
      (bind _output (`|GetArrayItem` (`self.AmmoStorage`) _ammoindex))
      (bind (_ammotype _currentammo _maxammo _binfinite) (break `/Game/GenericShooter/Addons/WeaponSystem/Core/FWeaponAmmoStorage` _output))
      ;[1 1 1] Grab ammo info, add delta to current ammo, return underflow.
      (if _binfinite
        (`self.OnAmmoChanged`)
        (return 0)
        (else
          (bind _output_get (set `local.FinalAmmoDelta` (`KismetMathLibrary.Min` _currentammo _ammodelta)))
          (setmembers `/Game/GenericShooter/Addons/WeaponSystem/Core/FWeaponAmmoStorage` :`StructRef` _output :`CurrentAmmo` (- _currentammo _output_get))
          (`self.OnAmmoChanged`)
          (return (`KismetMathLibrary.Max` (- _ammodelta (`local.FinalAmmoDelta`))))))
      (else
        (`KismetSystemLibrary.PrintText` (`|FormatText` "{Parent}: {Me} tried consuming {Amount} ammo for type {Type} but LooseAmmo does not have an element that defines ammo for {Type}." (`KismetTextLibrary.Conv_StringToText` (`KismetSystemLibrary.GetObjectName` (`self.GetOwner`))) (`KismetTextLibrary.Conv_StringToText` (`KismetSystemLibrary.GetObjectName` self)) (`local.AmmoDelta`) (`KismetTextLibrary.Conv_StringToText` (`KismetStringLibrary.Conv_ByteToString` (`local.AmmoType`)))))
        (return (`local.AmmoDelta`))))
    (else
      (`KismetSystemLibrary.PrintText` (`|FormatText` "{Parent}: {Me} tried consuming a negative amount of ammo ({Amount}) for type {Type}. Please use ConsumeAmmo instead." (`KismetTextLibrary.Conv_StringToText` (`KismetSystemLibrary.GetObjectName` (`self.GetOwner`))) (`KismetTextLibrary.Conv_StringToText` (`KismetSystemLibrary.GetObjectName` self)) (`local.AmmoDelta`) (`KismetTextLibrary.Conv_StringToText` (`KismetStringLibrary.Conv_ByteToString` (`local.AmmoType`)))))
      (return (`local.AmmoDelta`)))))

(fn `GetAmmoInfoForAmmoType`
  (params (AmmoType :type "/Game/GenericShooter/Addons/WeaponSystem/Core/EWeaponAmmoType Enum" :default "NewEnumerator3"))
  (returns (AmmoInfo :type "/Game/GenericShooter/Addons/WeaponSystem/Core/FWeaponAmmoStorage Structure") (AmmoIndex :type Integer) (bHasAmmoInfo :type Boolean))
  (for (_array_element _array_index) (`self.AmmoStorage`)
    (if (`|EnumEquality` (`.AmmoType_2_48D144044C0CAB70172228887222BD72` (break `/Game/GenericShooter/Addons/WeaponSystem/Core/FWeaponAmmoStorage` _array_element)) (`local.AmmoType`))
      (return _array_element _array_index true)))
  (return (make `/Game/GenericShooter/Addons/WeaponSystem/Core/FWeaponAmmoStorage` "NewEnumerator3") 0 false))

(fn `GetAmmoStorageCopy`
  (returns (AmmoStorage :type "Array of /Game/GenericShooter/Addons/WeaponSystem/Core/FWeaponAmmoStorage Structure"))
  (return (`self.AmmoStorage`)))

(fn `HasEnoughAmmo`
  (params (AmmoType :type "/Game/GenericShooter/Addons/WeaponSystem/Core/EWeaponAmmoType Enum" :default "NewEnumerator3") (Ammo :type Integer))
  (returns (bHasEnoughAmmo :type Boolean) (AvailableAmmo :type Integer))
  (bind _ammo (`local.Ammo`))
  (if (> Ammo 0)
    (bind (_ammoinfo _ammoindex _bhasammoinfo) (`self.GetAmmoInfoForAmmoType` AmmoType))
    (if _bhasammoinfo
      (bind (_ammotype _currentammo _maxammo _binfinite) (break `/Game/GenericShooter/Addons/WeaponSystem/Core/FWeaponAmmoStorage` _ammoinfo))
      (return (or (>= _currentammo _ammo) _binfinite) (`KismetMathLibrary.SelectInt` (`local.Ammo`) (`KismetMathLibrary.Min` _ammo _currentammo) _binfinite))
      (else
        (return false 0)))
    (else
      (return true 0))))

(fn `OnRep_AmmoStorage`
  (`self.OnAmmoChanged`)
  (return))

(fn `SetAmmo`
  (params (AmmoType :type "/Game/GenericShooter/Addons/WeaponSystem/Core/EWeaponAmmoType Enum" :default "NewEnumerator3") (CurrentAmmo :type Integer) (MaxAmmo :type Integer) (bSetMaxAmmo :type Boolean))
  (returns (bCreatedNewAmmoStorage :type Boolean))
  (bind (_ammoinfo _ammoindex _bhasammoinfo) (`self.GetAmmoInfoForAmmoType` AmmoType))
  (if _bhasammoinfo
    (bind _output (`|GetArrayItem` (`self.AmmoStorage`) _ammoindex))
    ;[1 1 1] Set ammo in already defined weapon ammo storage
    (setmembers `/Game/GenericShooter/Addons/WeaponSystem/Core/FWeaponAmmoStorage` :`StructRef` _output :`CurrentAmmo` (`local.CurrentAmmo`) :`MaxAmmo` (`KismetMathLibrary.SelectInt` (`local.MaxAmmo`) (`.MaxAmmo_7_D7CADF054DDFF08FE1AA6692803D306B` (break `/Game/GenericShooter/Addons/WeaponSystem/Core/FWeaponAmmoStorage` _output)) (`local.bSetMaxAmmo`)))
    (`self.OnAmmoChanged`)
    (return false)
    (else
      ;[1 1 1] If ammo type storage doesn't exist, add it.
      (`KismetArrayLibrary.Array_Add` (`self.AmmoStorage`) (make `/Game/GenericShooter/Addons/WeaponSystem/Core/FWeaponAmmoStorage` (`local.AmmoType`) (`local.CurrentAmmo`) (`KismetMathLibrary.SelectInt` (`local.MaxAmmo`) 0 (`local.bSetMaxAmmo`))))
      (`self.OnAmmoChanged`)
      (return true))))