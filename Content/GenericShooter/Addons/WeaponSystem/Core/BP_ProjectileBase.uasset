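; Base projectile actor for the weapon system that explodes with radial falloff damage on stopping, on bouncing off a pawn, or when destroyed, per its settings.
; The server applies damage and multicasts the impact effect through a found-or-spawned BP_WeaponReplicationHelper, while clients hide and deactivate their copy.
; Explosions without an impact reuse the cached stop hit, or trace along velocity (downward if nearly still) to generate one.
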(event `self.ReceiveBeginPlay`
  (`PrimitiveComponent.IgnoreActorWhenMoving` (`self.Mesh`) (`self.Instigator`) true))

(event `self.ProjectileMovement.OnProjectileStop`
  (params (ImpactResult :type "HitResult Structure (by ref)"))
  (if (`self.bExplodeOnProjectileStop`)
    (`self.ExplodeWithImpact` ImpactResult)
    (else
      (set `self.ProjectileStoppedImpactResult` ImpactResult))))

(event `self.ReceiveDestroyed`
  (if (and (not (`self.bExploded`)) (or (`KismetSystemLibrary.IsServer`) (`KismetSystemLibrary.IsStandalone`)))
    (`self.ExplodeWithoutImpact`)))

(event `self.ProjectileMovement.OnProjectileBounce`
  (params (ImpactResult :type "HitResult Structure (by ref)") (ImpactVelocity :type "Vector Structure (by ref)"))
  (if (`self.bExplodeWithImpactOnPawn`)
    (cast `Pawn` (`.HitActor` (`GameplayStatics.BreakHitResult` ImpactResult)))
    (`self.ExplodeWithImpact` ImpactResult)))

(fn `ClientSideQuietDeath`
  (if (`KismetMathLibrary.BooleanNOR` (`KismetSystemLibrary.IsServer`) (`KismetSystemLibrary.IsStandalone`))
    (`ActorComponent.Deactivate` (`self.ProjectileMovement`))
    (`SceneComponent.SetHiddenInGame` (`self.Mesh`) true true)
    (`self.SetActorEnableCollision` false)
    (return)
    (else
      (`VisualLoggerKismetLibrary.LogText` "Projectile called ClientSideQuietDeath on Server")
      (return))))

(fn `ExplodeWithImpact`
  (params (HitInfo :type "HitResult Structure"))
  (if (not (`self.bExploded`))
    (set `self.bExploded` true)
    (if (or (`KismetSystemLibrary.IsServer`) (`KismetSystemLibrary.IsStandalone`))
      (`self.LogDebugString` (`KismetStringLibrary.Concat_StrStr` "Projectile impacted with " (`KismetSystemLibrary.GetDisplayName` (`.HitActor` (`GameplayStatics.BreakHitResult` HitInfo))))
        (:`Out`
          (`/Game/GenericShooter/Addons/WeaponSystem/Core/BP_WeaponReplicationHelper.MulticastSpawnImpactEffect` (`self.GetWeaponReplicationActorOnServer`) (`self.ImpactEffectClass`) (`local.HitInfo`) (`self.GetInstigator`))
          (`GameplayStatics.ApplyRadialDamageWithFalloff` :`BaseDamage` (`self.BaseDamage`) :`MinimumDamage` (`self.MinimumDamage`) :`Origin` (`.ImpactPoint` (`GameplayStatics.BreakHitResult` (`local.HitInfo`))) :`DamageInnerRadius` (`self.DamageInnerRadius`) :`DamageOuterRadius` (`self.DamageOuterRadius`) :`DamageFalloff` (`self.DamageFalloff`) :`DamageTypeClass` (`self.DamageTypeClass`) :`DamageCauser` self :`InstigatedByController` (`self.GetInstigatorController`) :`DamagePreventionChannel` (`self.DamagePreventionChannel`))
          (`self.K2_DestroyActor`)
          (return)))
      (else
        (`self.ClientSideQuietDeath`)
        (return)))))

(fn `ExplodeWithoutImpact`
  (locals (FinalImpactResult :type "HitResult Structure"))
  (bind _returnvalue (`self.GetVelocity`))
  (bind _returnvalue_2 (`self.K2_GetActorLocation`))
  (bind _finalimpactresult (`local.FinalImpactResult`))
  (if (not (`self.bExploded`))
    (set `self.bExploded` true)
    (if (or (`KismetSystemLibrary.IsServer`) (`KismetSystemLibrary.IsStandalone`))
      (if (`GameplayStatics.BreakHitResult` (`self.ProjectileStoppedImpactResult`))
        (set `local.FinalImpactResult` (`self.ProjectileStoppedImpactResult`))
        (`self.LogDebugString` "Exploding without impact, using cached impact from projectile stopping."
          (:`Out`
            _))
        (else
          (`self.LogDebugString` "Exploding without impact, attempting to generate impact info."
            (:`Out`
              (bind _outhit (`KismetSystemLibrary.LineTraceSingle` :`Start` _returnvalue_2 :`End` (`KismetMathLibrary.SelectVector` (+ _returnvalue_2 (0.0 0.0 -15.0)) (+ _returnvalue_2 (* _returnvalue 0.05)) (<= (`KismetMathLibrary.VSizeSquared` _returnvalue) 64.0)) :`TraceChannel` "TraceTypeQuery1" :`DrawDebugType` (select `bool` (`self.bDebug`) :`true` "Persistent" :!type "EDrawDebugTrace Enum")))
              (set `local.FinalImpactResult` _outhit)))))
      (`/Game/GenericShooter/Addons/WeaponSystem/Core/BP_WeaponReplicationHelper.MulticastSpawnImpactEffect` (`self.GetWeaponReplicationActorOnServer`) (`self.ImpactEffectClass`) _finalimpactresult (`self.GetInstigator`))
      (`GameplayStatics.ApplyRadialDamageWithFalloff` :`BaseDamage` (`self.BaseDamage`) :`MinimumDamage` (`self.MinimumDamage`) :`Origin` (`.Location` (`GameplayStatics.BreakHitResult` _finalimpactresult)) :`DamageInnerRadius` (`self.DamageInnerRadius`) :`DamageOuterRadius` (`self.DamageOuterRadius`) :`DamageFalloff` (`self.DamageFalloff`) :`DamageTypeClass` (`self.DamageTypeClass`) :`DamageCauser` self :`InstigatedByController` (`self.GetInstigatorController`) :`DamagePreventionChannel` (`self.DamagePreventionChannel`))
      (`self.K2_DestroyActor`)
      (return)
      (else
        (`self.ClientSideQuietDeath`)
        (return)))))

(fn `GetUserFriendlyNameThroughInterface`
  (returns (DisplayName :type Text))
  (return (`self.UserFriendlyName`)))

(fn `GetWeaponReplicationActorOnServer`
  (returns (Helper :type "/Game/GenericShooter/Addons/WeaponSystem/Core/BP_WeaponReplicationHelper Object Reference"))
  (if (or (`KismetSystemLibrary.IsServer`) (`KismetSystemLibrary.IsStandalone`))
    (bind _outactors (`GameplayStatics.GetAllActorsOfClass` "/Game/GenericShooter/Addons/WeaponSystem/Core/BP_WeaponReplicationHelper.BP_WeaponReplicationHelper_C"))
    (if (`KismetArrayLibrary.Array_IsValidIndex` _outactors)
      (return (`|GetArrayItem` _outactors))
      (else
        (bind _returnvalue (`|SpawnActorFromClass` "/Game/GenericShooter/Addons/WeaponSystem/Core/BP_WeaponReplicationHelper.BP_WeaponReplicationHelper_C" (`KismetMathLibrary.MakeTransform` (0.0 0.0 0.0)) "AlwaysSpawn" "OverrideRootScale" null null))
        (return _returnvalue)))
    (else
      (return null))))

(fn `UserConstructionScript`
  (bind _breplicateprojectilemovement (`self.bReplicateProjectileMovement`))
  (`self.SetReplicateMovement` _breplicateprojectilemovement)
  (`ActorComponent.SetIsReplicated` (`self.ProjectileMovement`) _breplicateprojectilemovement)
  (`ActorComponent.SetIsReplicated` (`self.Mesh`) _breplicateprojectilemovement))