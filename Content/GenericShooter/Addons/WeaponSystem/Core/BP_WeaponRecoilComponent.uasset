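; Weapon component that computes horizontal and vertical recoil spread for each shot of its owning pawn.
; PerformRecoilAttack returns spread from the current factor, then raises that factor and refreshes a sustain timer.
; Spread samples a scaled curve from SpreadConfig, then chains ADS, velocity, in-air and crouch modifiers, the latter three additive or multiplicative.
; Tick decays the factor once the sustain time expires, carrying over the frame's leftover time.
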(event EventTick
  (params (DeltaSeconds :type Float%20%28single-precision%29))
  (CallFunction|UpdateSpreadFactor DeltaSeconds))

(fn PerformRecoilAttack
  (params (SpreadFactorIncrease :type Float%20%28single-precision%29) (ADSPosition :type Float%20%28single-precision%29))
  (Utilities|FlowControl|Sequence
    (:then_0
      (bind (_horizontalspread _verticalspread) (CallFunction|CalculateCurrentSpread ADSPosition))
      (LocalVariables|SetOutputSpread (Math|Vector|MakeVector _horizontalspread _verticalspread 0.0)))
    (:then_1
      (Variables|Default|SetCurrentSpreadFactor (Math|Float|Clamp(Float) (+ (Variables|Default|GetCurrentSpreadFactor) SpreadFactorIncrease)))
      (Variables|Default|SetRemainingSustainTime (Math|Float|Max(Float) (Utilities|Struct|BreakFWeaponRecoilConfig (Variables|Default|GetSpreadConfig)) (Variables|Default|GetRemainingSustainTime))))
    (:then_2
      (return (.X (Math|Vector|BreakVector (LocalVariables|GetOutputSpread))) (.Y (Math|Vector|BreakVector (LocalVariables|GetOutputSpread)))))))

(fn UpdateSpreadFactor
  (params (DeltaSeconds :type Float%20%28single-precision%29))
  (if (> (Variables|Default|GetCurrentSpreadFactor) 0.0)
    (Utilities|FlowControl|Sequence
      (:then_0
        (if (> (Variables|Default|GetRemainingSustainTime) 0.0)
          (if (< (- (Variables|Default|GetRemainingSustainTime) DeltaSeconds) 0.0)
            (Variables|Default|SetRemainingSustainTime 0.0)
            (LocalVariables|SetCalculatedDecay (|((Abs(({A3C90C35-477C-DA23-47AB-5FAA0B007D87}-DeltaSeconds)))*DecayRate) DeltaSeconds (Utilities|Struct|BreakFWeaponRecoilConfig (Variables|Default|GetSpreadConfig))))
            (else
              (return)))
          (else
            (LocalVariables|SetCalculatedDecay (* (Utilities|Struct|BreakFWeaponRecoilConfig (Variables|Default|GetSpreadConfig)) DeltaSeconds)))))
      (:then_1
        (Variables|Default|SetCurrentSpreadFactor (- (Variables|Default|GetCurrentSpreadFactor) (LocalVariables|GetCalculatedDecay)))
        (return)))
    (else
      (return))))

(fn SetRecoilConfig
  (params (NewSpreadCurve :type F%20Weapon%20Recoil%20Config%20Structure) (OwningPawn :type Pawn%20Object%20Reference))
  (bind _returnvalue (Utilities|String|MakeLiteralString "ERROR: WeaponRecoilComponent had SetRecoilConfig called without a valid owning Pawn!"))
  (Utilities|DebugPrintMacro "SetRecoilConfig called.")
  (Utilities|FlowControl|Sequence
    (:then_0
      (Variables|Default|SetOwningPawn OwningPawn)
      (Variables|Default|SetSpreadConfig NewSpreadCurve)
      (CallFunction|ResetSpread))
    (:then_1
      (Variables|Default|GetOwningPawn
        (:then)
        (:else
          (Development|PrintString _returnvalue)
          (Class|VisualLoggerKismetLibrary|LogText _returnvalue "Blueprint Log"))))
    (:then_2
      (return))))

(fn ResetSpread
  (Variables|Default|SetCurrentSpreadFactor 0.0)
  (Variables|Default|SetRemainingSustainTime 0.0)
  (return))

(fn CalculateCurrentSpread
  (params (ADSPosition :type Float%20%28single-precision%29))
  (bind _newspread (CallFunction|ApplyADSModifier ADSPosition (CallFunction|GetBaseSpreadValue)))
  (bind _newspread_2 (CallFunction|ApplyVelocityModifier _newspread))
  (bind _newspread_3 (CallFunction|ApplyAirModifier _newspread_2))
  (bind _newspread_4 (CallFunction|ApplyCrouchingModifier _newspread_3))
  (return (.X (Math|Vector|BreakVector _newspread_4)) (.Y (Math|Vector|BreakVector _newspread_4))))

(fn ApplyCrouchingModifier
  (params (Spread :type Vector%20%28by%20ref%29))
  (bind _spreadconfig (Variables|Default|GetSpreadConfig))
  (bind (_ownercrouchingspreadmodifier _ownercrouchingspreadmodifierisadditive) (Utilities|Struct|BreakFWeaponRecoilConfig _spreadconfig))
  (bind _returnvalue (+ Spread _ownercrouchingspreadmodifier))
  (bind _returnvalue_2 (* Spread _ownercrouchingspreadmodifier))
  (bind _owningpawn (Variables|Default|GetOwningPawn)
    (:then
      (Utilities|IsValid (Pawn|GetMovementComponent _owningpawn)
        (:Is%20Valid
          (if (AI|Components|NavMovement|IsCrouching (Pawn|GetMovementComponent _owningpawn))
            (if _ownercrouchingspreadmodifierisadditive
              (Utilities|DebugPrintSpreadMacro Spread "Crouching" _returnvalue)
              (|SetBy-RefVar Spread _returnvalue)
              (else
                (Utilities|DebugPrintSpreadMacro Spread "Crouching" _returnvalue_2)
                (|SetBy-RefVar Spread _returnvalue_2)))
            (return Spread)
            (else
              _)))
        (:Is%20Not%20Valid
          _))
      (return Spread))
    (:else
      (return Spread))))

(fn ApplyAirModifier
  (params (Spread :type Vector%20%28by%20ref%29))
  (bind _spreadconfig (Variables|Default|GetSpreadConfig))
  (bind (_ownerinairspreadmodifier _ownerinairspreadmofifierisadditive) (Utilities|Struct|BreakFWeaponRecoilConfig _spreadconfig))
  (bind _returnvalue (+ Spread _ownerinairspreadmodifier))
  (bind _returnvalue_2 (* Spread _ownerinairspreadmodifier))
  (bind _owningpawn (Variables|Default|GetOwningPawn)
    (:then
      (Utilities|IsValid (Pawn|GetMovementComponent _owningpawn)
        (:Is%20Valid
          (if (not (AI|Components|NavMovement|IsMovingonGround (Pawn|GetMovementComponent _owningpawn)))
            (if _ownerinairspreadmofifierisadditive
              (Utilities|DebugPrintSpreadMacro Spread "Air" _returnvalue)
              (|SetBy-RefVar Spread _returnvalue)
              (else
                (Utilities|DebugPrintSpreadMacro Spread "Air" _returnvalue_2)
                (|SetBy-RefVar Spread _returnvalue_2)))
            (return Spread)
            (else
              _)))
        (:Is%20Not%20Valid
          _))
      (return Spread))
    (:else
      (return Spread))))

(fn ApplyVelocityModifier
  (params (Spread :type Vector%20%28by%20ref%29))
  (bind _spreadconfig (Variables|Default|GetSpreadConfig))
  (bind (_ownervelocityspreadmodifier _ownervelocityspreadmodifierisadditive) (Utilities|Struct|BreakFWeaponRecoilConfig _spreadconfig))
  (bind _owningpawn (Variables|Default|GetOwningPawn)
    (:then
      (if _ownervelocityspreadmodifierisadditive
        (Utilities|DebugPrintSpreadMacro Spread "Velocity" (+ Spread (Math|Curves|GetFloatValue _ownervelocityspreadmodifier (Math|Vector|VectorLength (Transformation|GetVelocity _owningpawn)))))
        (|SetBy-RefVar Spread (+ Spread (Math|Curves|GetFloatValue _ownervelocityspreadmodifier (Math|Vector|VectorLength (Transformation|GetVelocity _owningpawn)))))
        (else
          (Utilities|DebugPrintSpreadMacro Spread "Velocity" (* Spread (Math|Curves|GetFloatValue _ownervelocityspreadmodifier (Math|Vector|VectorLength (Transformation|GetVelocity _owningpawn)))))
          (|SetBy-RefVar Spread (* Spread (Math|Curves|GetFloatValue _ownervelocityspreadmodifier (Math|Vector|VectorLength (Transformation|GetVelocity _owningpawn)))))))
      (return Spread))
    (:else
      (return Spread))))

(fn ApplyADSModifier
  (params (ADSPosition :type Float%20%28single-precision%29) (Spread :type Vector%20%28by%20ref%29))
  (bind _spreadconfig (Variables|Default|GetSpreadConfig))
  (bind _owneradsspreadmodifier (Utilities|Struct|BreakFWeaponRecoilConfig _spreadconfig))
  (bind _returnvalue (Math|Curves|GetFloatValue _owneradsspreadmodifier ADSPosition))
  (bind _returnvalue_2 (* Spread _returnvalue))
  (Utilities|IsValid _owneradsspreadmodifier
    (:Is%20Valid
      (Utilities|DebugPrintSpreadMacro Spread "ADS" _returnvalue_2)
      (|SetBy-RefVar Spread _returnvalue_2)
      (return Spread))
    (:Is%20Not%20Valid
      (return Spread))))

(fn GetBaseSpreadValue
  (bind _spreadconfig (Variables|Default|GetSpreadConfig))
  (bind _currentspreadfactor (Variables|Default|GetCurrentSpreadFactor))
  (bind (_spreadcurve _spreadcurvescale) (Utilities|Struct|BreakFWeaponRecoilConfig _spreadconfig))
  (bind _returnvalue (Math|Curves|GetVectorValue _spreadcurve _currentspreadfactor))
  (bind _returnvalue_2 (* _returnvalue _spreadcurvescale))
  (Utilities|IsValid _spreadcurve
    (:Is%20Valid
      (Utilities|DebugPrintSpreadMacro :ModifierName "Base" :ModifiedSpread _returnvalue_2)
      (return _returnvalue_2))
    (:Is%20Not%20Valid
      (Development|PrintString "ERROR: WeaponRecoilComponent tried calculating spread without a spread curve!" true true "(R=1.000000,G=0.040325,B=0.000000,A=1.000000)")
      (return "0, 0, 0"))))