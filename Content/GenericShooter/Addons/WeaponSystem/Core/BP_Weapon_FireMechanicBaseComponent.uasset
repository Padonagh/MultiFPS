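; Base weapon component for fire mechanics, handling shot timing, ammo checks, muzzle effects and an empty PerformMechanic hook.
; On BeginPlay it caches tagged meshes, muzzle flash and audio components, and loaded ammo storage from the owner.
; StartFire and StopFire run locally and route to the server; automatic fire re-arms a timer, optionally adding ping-based delay on clients.
; Helpers provide aim from eyes or muzzle, seeded cone spread, ammo consumption and debug logging.
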(event Custom|ServerStartFire
  (CallFunction|StartFire))

(event Custom|ServerStopFire
  (CallFunction|StopFire))

(event EventBeginPlay
  (CallFunction|CacheMeshes)
  (CallFunction|CacheLoadedAmmoStorage)
  (CallFunction|CacheMuzzleFlashComponents)
  (CallFunction|CacheMuzzleAudioComponents))

(fn CacheMeshes
  (bind _returnvalue (Components|GetOwner))
  (bind _returnvalue_2 (Components|GetOwner))
  (bind _weaponfirstpersonmeshtag (Variables|Config|WeaponInfo|GetWeaponFirstPersonMeshTag))
  (bind _weaponthirdpersonmeshtag (Variables|Config|WeaponInfo|GetWeaponThirdPersonMeshTag))
  (bind _returnvalue_3 (Actor|GetComponentsbyTag _returnvalue "/Script/Engine.SkeletalMeshComponent" _weaponthirdpersonmeshtag))
  (bind _returnvalue_4 (Actor|GetComponentsbyTag _returnvalue_2 "/Script/Engine.SkeletalMeshComponent" _weaponfirstpersonmeshtag))
  (Utilities|FlowControl|Sequence
    (:then_0
      (if (> (Utilities|Array|Length _returnvalue_4) 0)
        (Variables|Default|SetFirstPersonMesh (Utilities|Array|Get(acopy) _returnvalue_4))))
    (:then_1
      (if (> (Utilities|Array|Length _returnvalue_3) 0)
        (Variables|Default|SetThirdPersonMesh (Utilities|Array|Get(acopy) _returnvalue_3))))
    (:then_2
      (return))))

(fn GetAim
  (bind _returnvalue (Components|GetOwner))
  (bind _thirdpersonmesh (Variables|Default|GetThirdPersonMesh))
  (bind _thirdpersonmuzzlesocket (Variables|Config|WeaponInfo|GetThirdPersonMuzzleSocket))
  (bind _firstpersonmesh (Variables|Default|GetFirstPersonMesh))
  (bind _firstpersonmuzzlesocket (Variables|Config|WeaponInfo|GetFirstPersonMuzzleSocket))
  (bind _returnvalue_2 (Transformation|GetSocketTransform _thirdpersonmesh _thirdpersonmuzzlesocket "RTS_World"))
  (bind _returnvalue_3 (Components|GetOwner _returnvalue))
  (bind _returnvalue_4 (Transformation|GetSocketTransform _firstpersonmesh _firstpersonmuzzlesocket "RTS_World"))
  (bind _outlocation (Actor|GetActorEyesViewPoint _returnvalue_3))
  (bind _endpoint (Class|BPIWeaponSystemHolder|GetWorldAimEndPoint(Message) (CallFunction|GetOwnerOwnerasPawn)))
  (LocalVariables|SetLocalEndPoint _endpoint)
  (switch Utilities|FlowControl|Switch|SwitchonECharacterAimPoint (Variables|Config|Mechanic|GetGetAimLocationType)
    (:NewEnumerator3
      (return _outlocation (Math|Rotator|FindLookatRotation _outlocation (LocalVariables|GetLocalEndPoint))))
    (:NewEnumerator1
      (return (.location _returnvalue_2) (Math|Rotator|FindLookatRotation (.location _returnvalue_2) (LocalVariables|GetLocalEndPoint))))
    (:NewEnumerator2
      (return (.location _returnvalue_4) (Math|Rotator|FindLookatRotation (.location _returnvalue_4) (LocalVariables|GetLocalEndPoint))))))

(fn SpawnMuzzleFlash
  (bind _muzzlepsc (CallFunction|GetCurrentMuzzle))
  (Utilities|IsValid _muzzlepsc
    (:Is%20Valid
      (Components|Activation|Activate _muzzlepsc true)
      (return))
    (:Is%20Not%20Valid
      (return))))

(fn CacheMuzzleFlashComponents
  (bind _returnvalue (Components|GetOwner))
  (bind _returnvalue_2 (Components|GetOwner))
  (bind _firstpersonmuzzleflashcomponenttag (Variables|Config|WeaponInfo|GetFirstPersonMuzzleFlashComponentTag))
  (bind _thirdpersonmuzzleflashcomponenttag (Variables|Config|WeaponInfo|GetThirdPersonMuzzleFlashComponentTag))
  (bind _returnvalue_3 (Actor|GetComponentsbyTag _returnvalue "/Script/Engine.ParticleSystemComponent" _thirdpersonmuzzleflashcomponenttag))
  (bind _returnvalue_4 (Actor|GetComponentsbyTag _returnvalue_2 "/Script/Engine.ParticleSystemComponent" _firstpersonmuzzleflashcomponenttag))
  (Utilities|FlowControl|Sequence
    (:then_0
      (if (> (Utilities|Array|Length _returnvalue_4) 0)
        (Variables|Default|SetFirstPersonMuzzleFlashComponent (Utilities|Array|Get(acopy) _returnvalue_4))))
    (:then_1
      (if (> (Utilities|Array|Length _returnvalue_3) 0)
        (Variables|Default|SetThirdPersonMuzzleFlashComponent (Utilities|Array|Get(acopy) _returnvalue_3))))
    (:then_2
      (return))))

(fn GetCurrentMuzzle
  (return (Transformation|GetSocketTransform (.AsSkeletal%20Mesh%20Component (Utilities|Casting|CastToSkeletalMeshComponent (Utilities|SelectObject (Variables|Default|GetThirdPersonMesh) (Variables|Default|GetFirstPersonMesh) (Variables|Default|GetbUseThirdPersonVisuals)))) (select (Variables|Default|GetbUseThirdPersonVisuals) (Variables|Config|WeaponInfo|GetThirdPersonMuzzleSocket) (Variables|Config|WeaponInfo|GetFirstPersonMuzzleSocket)) "RTS_World") (select (Variables|Default|GetbUseThirdPersonVisuals) (Variables|Default|GetThirdPersonMuzzleFlashComponent) (Variables|Default|GetFirstPersonMuzzleFlashComponent)) (select (Variables|Default|GetbUseThirdPersonVisuals) (Variables|Default|GetThirdPersonMuzzleAudio) (Variables|Default|GetFirstPersonMuzzleAudio))))

(fn StartFire
  (bind (_bcanfire _btryrefire) (CallFunction|CanFire))
  (if (Networking|IsServer)
    _
    (else
      (CallFunction|ServerStartFire)))
  (Variables|Default|SetbWantsToFire true)
  (if _bcanfire
    (CallFunction|Fire)
    (return)
    (elif _btryrefire
      (CallFunction|SetTimerforNextShot)
      (return)
      (else
        (return)))))

(fn StopFire
  (Utilities|PrintDebugInfo "Mechanic calling Stop Fire."
    (:Out
      (if (Utilities|Name|NotEqual(Name) (Variables|Config|Animation|GetFireAnimEndSection) "None")
        (Default|CallOnRequestPlayWeaponAnimation self (Variables|Config|Animation|GetFireAnimKeyName) 0.0 (Variables|Config|Animation|GetFireAnimEndSection) false) ; Tell fire montage to skip to end if end section is provided
      )
      (if (Networking|IsServer)
        _
        (else
          (Utilities|IsValid (Components|GetOwner)
            (:Is%20Valid
              (Utilities|PrintDebugInfo "Mechanic routing Stop Fire to Server."
                (:Out
                  (CallFunction|ServerStopFire))))
            (:Is%20Not%20Valid
              (return)))))
      (Variables|Default|SetbWantsToFire false)
      (Utilities|Time|ClearandInvalidateTimerbyHandle (Variables|Default|GetFireTimerHandle))
      (Default|CallOnStopFire false)
      (return))))

(fn CanFire
  (bind _bhasloadedammo (CallFunction|HasAmmoLoaded))
  (bind _returnvalue (CallFunction|HasEnoughTimePassedBetweenShots))
  (return (and _returnvalue _bhasloadedammo) (Math|Boolean|ANDBoolean (not _returnvalue) (Variables|Config|Mechanic|GetbAutomatic) _bhasloadedammo)))

(fn Fire
  (bind (_bcanfire _btryrefire) (CallFunction|CanFire))
  (bind _self self)
  (if (and _bcanfire (Variables|Default|GetbWantsToFire))
    (Default|CallOnPreFire _self false)
    (Default|CallOnRequestPlayWeaponAnimation _self (Variables|Config|Animation|GetFireAnimKeyName) 0.0 "" false)
    (CallFunction|UpdateShouldUseThirdPersonVisuals)
    (Utilities|PrintDebugInfo "Fire determined it should perform mechanic."
      (:Out
        (CallFunction|PerformMechanic)
        (CallFunction|SpawnMuzzleFlash)
        (CallFunction|PlayFireSound)
        (Math|Integer|IncrementInt (Variables|Default|GetShotCount)
          (:%20%20
            (Variables|Default|SetLastShootTime (+ (Utilities|Time|GetGameTimeinSeconds) (CallFunction|GetClientSidePredictedShootDelay)))
            (Default|CallOnPostFire self false)
            (if (Variables|Config|Mechanic|GetbAutomatic)
              (Utilities|PrintDebugInfo "Fire successfully fired and is now trying to refire."
                (:Out
                  (CallFunction|SetTimerforNextShot)
                  (return)))
              (else
                (Utilities|PrintDebugInfo "Fire successfully fired but is not automatic, calling Stop Fire."
                  (:Out
                    (CallFunction|StopFire)
                    (return)))))))))
    (elif _btryrefire
      (Utilities|PrintDebugInfo "Fire determined it should refire."
        (:Out
          (CallFunction|SetTimerforNextShot)
          (return)))
      (else
        (Utilities|PrintDebugInfo "Fire determined it should NOT refire."
          (:Out
            (return)))))))

(fn CacheMuzzleAudioComponents
  (bind _returnvalue (Components|GetOwner))
  (bind _returnvalue_2 (Components|GetOwner))
  (bind _firstpersonmuzzleaudiocomponenttag (Variables|Config|WeaponInfo|GetFirstPersonMuzzleAudioComponentTag))
  (bind _thirdpersonmuzzleaudiocomponenttag (Variables|Config|WeaponInfo|GetThirdPersonMuzzleAudioComponentTag))
  (bind _returnvalue_3 (Actor|GetComponentsbyTag _returnvalue "/Script/Engine.AudioComponent" _thirdpersonmuzzleaudiocomponenttag))
  (bind _returnvalue_4 (Actor|GetComponentsbyTag _returnvalue_2 "/Script/Engine.AudioComponent" _firstpersonmuzzleaudiocomponenttag))
  (Utilities|FlowControl|Sequence
    (:then_0
      (if (> (Utilities|Array|Length _returnvalue_4) 0)
        (Variables|Default|SetFirstPersonMuzzleAudio (Utilities|Array|Get(acopy) _returnvalue_4))))
    (:then_1
      (if (> (Utilities|Array|Length _returnvalue_3) 0)
        (Variables|Default|SetThirdPersonMuzzleAudio (Utilities|Array|Get(acopy) _returnvalue_3))))
    (:then_2
      (return))))

(fn PlayFireSound
  (bind _muzzleaudio (CallFunction|GetCurrentMuzzle))
  (bind _firesound (Variables|Config|Audio|GetFireSound)
    (:then
      (if (!= _firesound (Variables|/Script/Engine.AudioComponent|GetSound _muzzleaudio))
        (Audio|Components|Audio|SetSound _muzzleaudio (Variables|Config|Audio|GetFireSound)))
      (Audio|Components|Audio|Play _muzzleaudio 0.0)
      (return))
    (:else
      (return))))

(fn PerformMechanic
  (return))

(fn UpdateShouldUseThirdPersonVisuals
  (Variables|Default|SetbUseThirdPersonVisuals (not (Rendering|IsVisible (Variables|Default|GetFirstPersonMesh))))
  (return))

(fn GetClientSidePredictedShootDelay
  (bind _returnvalue (Game|GetPlayerController 0))
  (if (and (not (Networking|IsServer)) (Variables|Default|GetbUseClientSidePredictedShootDelay))
    (Utilities|IsValid _returnvalue
      (:Is%20Valid
        (bind _playerstate (Variables|/Script/Engine.Controller|GetPlayerState _returnvalue)
          (:then
            (return (/ (Math|Conversions|ToFloat(Integer) (* (Math|Conversions|ToInteger(Byte) (Variables|/Script/Engine.PlayerState|GetPing _playerstate)) 4)) 1e+03)))
          (:else
            (return 0.0))))
      (:Is%20Not%20Valid
        (return 0.0)))
    (else
      (return 0.0))))

(fn HasEnoughTimePassedBetweenShots
  (bind _returnvalue (Utilities|Time|GetGameTimeinSeconds))
  (bind _lastshoottime (Variables|Default|GetLastShootTime))
  (bind _timebetweenshots (Variables|Config|Mechanic|Timing|GetTimeBetweenShots))
  (bind _returnvalue_2 (- _returnvalue _lastshoottime))
  (return (or (>= _returnvalue_2 _timebetweenshots) (Math|Float|NearlyEqual(Float) _returnvalue_2 _timebetweenshots (Variables|Config|Mechanic|Timing|GetTimeBetweenShotsErrorTolerance)))))

(fn TimeUntilNextShot
  (return (Math|Float|Max(Float) (- (+ (Variables|Default|GetLastShootTime) (Variables|Config|Mechanic|Timing|GetTimeBetweenShots)) (Utilities|Time|GetGameTimeinSeconds)) 0.0)))

(fn SetTimerforNextShot
  (bind _returnvalue (Utilities|Time|SetTimerbyEvent (EventDispatchers|CreateEvent :!event Fire) (CallFunction|TimeUntilNextShot)))
  (Variables|Default|SetFireTimerHandle _returnvalue)
  (return))

(fn Reload
  (return))

(fn CanReload
  (return true))

(fn HasAmmoLoaded
  (Utilities|IsValid (Utilities|ToObject(Interface) (Variables|Default|GetLoadedAmmoStorage))
    (:Is%20Valid
      (bind _bhasenoughammo (Default|HasEnoughAmmo (Variables|Default|GetLoadedAmmoStorage) (Variables|Config|Ammo|GetAmmoType) (Variables|Config|Ammo|GetConsumeAmmoCount)))
      (return _bhasenoughammo))
    (:Is%20Not%20Valid
      (return false))))

(fn CacheLoadedAmmoStorage
  (bind _returnvalue (Components|GetOwner))
  (bind _loadedammostoragetag (Variables|Config|WeaponInfo|GetLoadedAmmoStorageTag))
  (bind _returnvalue_2 (Actor|GetComponentsbyTag _returnvalue "/Script/Engine.ActorComponent" _loadedammostoragetag))
  (if (> (Utilities|Array|Length _returnvalue_2) 0)
    (bind _asbpi_generic_ammo_storage (Utilities|Casting|CastToBPI_GenericAmmoStorage (Utilities|Array|Get(acopy) _returnvalue_2))
      (:then
        (Variables|Default|SetLoadedAmmoStorage _asbpi_generic_ammo_storage)
        (return))
      (:CastFailed
        _)))
  (Development|PrintText (Utilities|Text|FormatText "ERROR: {Me} failed to cache its loaded ammo storage." (Utilities|Text|ToText(String) (Utilities|GetObjectName self))) true true "(R=1.000000,G=0.056108,B=0.000000,A=1.000000)" 1e+01)
  (return))

(fn ConsumeAmmo
  (bind _consumeammocount (Variables|Config|Ammo|GetConsumeAmmoCount))
  (Utilities|IsValid (Utilities|ToObject(Interface) (Variables|Default|GetLoadedAmmoStorage))
    (:Is%20Valid
      (bind _ammounderflow (Default|ConsumeAmmo (Variables|Default|GetLoadedAmmoStorage) (Variables|Config|Ammo|GetAmmoType) _consumeammocount))
      (return (< _ammounderflow _consumeammocount)))
    (:Is%20Not%20Valid
      (return false))))

(fn GetAimVectorwithSpread
  (params (AimRot :type Rotator))
  (LocalVariables|SetHalfAngleRadians (|(((Vector2D(({8012F0FE-41E2-DB68-3DFD-BBA25C65068D}+{606DF9C5-4427-F598-1F5C-DF95237B8534}),({5A0F8C9E-4B96-7A6E-8780-2A86EEEA60DB}+{D7531922-4A67-D28A-8B88-99A7BEF68779})))/2)*0.017453)))
  (Utilities|PrintDebugInfo (Utilities|String|ToString(Text) (Utilities|Text|FormatText "GetAimVectorWithSpread: AimRot: {AimRot} Horz/Vert Spread: {HorzSpread} {VertSpread} Output Vector: {Output}" (Utilities|Text|ToText(String) AimRot) (.X (Math|Vector2D|BreakVector2D (LocalVariables|GetHalfAngleRadians))) (.Y (Math|Vector2D|BreakVector2D (LocalVariables|GetHalfAngleRadians))) (Utilities|Text|ToText(String) (CallFunction|GenericRandomUnitVectorinConefromStream (Variables|Default|GetRandomStream) (Math|Vector|Normalize (Math|Rotator|GetRotationXVector AimRot)) (.X (Math|Vector2D|BreakVector2D (LocalVariables|GetHalfAngleRadians))) (.Y (Math|Vector2D|BreakVector2D (LocalVariables|GetHalfAngleRadians)))))))
    (:Out
      (return (CallFunction|GenericRandomUnitVectorinConefromStream (Variables|Default|GetRandomStream) (Math|Vector|Normalize (Math|Rotator|GetRotationXVector AimRot)) (.X (Math|Vector2D|BreakVector2D (LocalVariables|GetHalfAngleRadians))) (.Y (Math|Vector2D|BreakVector2D (LocalVariables|GetHalfAngleRadians))))))))

(fn LogDamage
  (params (HitZoneName :type Name) (HitInfo :type Hit%20Result%20Structure) (Damage :type Float%20%28single-precision%29))
  (bind _returnvalue (Components|GetOwner))
  (bind (_bblockinghit _binitialoverlap _time _distance _location _impactpoint _normal _impactnormal _physmat _hitactor _hitcomponent _hitbonename) (Collision|BreakHitResult HitInfo))
  (bind _self self)
  (bind _returnvalue_2 (Utilities|GetDisplayName _hitactor))
  (bind _returnvalue_3 (Utilities|GetDisplayName _self))
  (bind _returnvalue_4 (Utilities|GetDisplayName _returnvalue))
  (bind _returnvalue_5 (Utilities|Text|ToText(Name) HitZoneName))
  (bind _returnvalue_6 (Utilities|Name|NotEqual(Name) HitZoneName "None"))
  (bind _returnvalue_7 (Utilities|Name|NotEqual(Name) _hitbonename "None"))
  (bind _returnvalue_8 (Utilities|Text|ToText(Name) _hitbonename))
  (bind _returnvalue_9 (Utilities|IsValid _hitcomponent))
  (bind _returnvalue_10 (Utilities|GetDisplayName _hitcomponent))
  (bind _returnvalue_11 (Utilities|Text|ToText(String) _returnvalue_2))
  (bind _returnvalue_12 (Utilities|Text|ToText(String) _returnvalue_3))
  (bind _returnvalue_13 (Utilities|Text|ToText(String) _returnvalue_4))
  (bind _returnvalue_14 (Utilities|Text|ToText(String) _returnvalue_10))
  (bind _result (Utilities|Text|FormatText " at bone: {BoneName}" _returnvalue_8))
  (bind _result_2 (Utilities|Text|FormatText " , hit zone: {HitZone}." _returnvalue_5))
  (bind _result_3 (Utilities|Text|FormatText " on component {Component}" _returnvalue_14))
  (bind _returnvalue_15 (select _returnvalue_6 _result_2 "."))
  (bind _returnvalue_16 (select _returnvalue_7 _result ""))
  (bind _returnvalue_17 (select _returnvalue_9 _result_3 "."))
  (bind _result_4 (Utilities|Text|FormatText "DEBUG: {Me} of {Weapon} dealt {Damage} damage to {DamagedActor}{ComponentInfo}{BoneInfo}{HitZoneInfo}" _returnvalue_12 _returnvalue_13 Damage _returnvalue_11 _returnvalue_17 _returnvalue_16 _returnvalue_15))
  (bind _returnvalue_18 (Utilities|String|ToString(Text) _result_4))
  (if (Variables|Config|Debug|GetbPrintDebugInfo)
    (Class|VisualLoggerKismetLibrary|LogLocation _impactpoint _returnvalue_18 "(R=0.122074,G=1.000000,B=0.000000,A=1.000000)" 1e+01 "Blueprint Log")
    (Development|PrintString _returnvalue_18 true true "(R=0.000000,G=0.466854,B=1.000000,A=1.000000)")
    (return)
    (else
      (return))))

(fn GetOwnerOwnerasPawn
  (return (.AsPawn (Utilities|Casting|CastToPawn (Components|GetOwner (Components|GetOwner))))))

(fn SetRecoilSpreadValues
  (params (HorizontalSpread :type Float%20%28single-precision%29) (VerticalSpread :type Float%20%28single-precision%29))
  (Variables|Default|SetRecoilHorizontalSpread HorizontalSpread)
  (Variables|Default|SetRecoilVerticalSpread VerticalSpread)
  (return))