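; BP_WeaponProxy_Base is the base world pickup for a weapon, a focusable interactable that shows the item's friendly name.
; On BeginPlay it spawns a default item info actor on server or standalone if none is set, and can launch its mesh with physics and a throw impulse.
; Interacting adds that item info to the interactor's slot inventory component and destroys the proxy on success, printing errors for invalid cases.
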(event `self.ReceiveBeginPlay`
  (bind _weaponmesh (`self.WeaponMesh`))
  (`self.CreateItemInfoIfMissing`)
  (if (`self.bSimulatePhysicsOnBeginPlay`)
    (`PrimitiveComponent.SetCollisionEnabled` _weaponmesh "QueryAndPhysics")
    (`PrimitiveComponent.SetSimulatePhysics` _weaponmesh true)
    (`PrimitiveComponent.AddImpulse` (`self.WeaponMesh`) (`self.InitialThrowVelocity`) "None" true)))

(event `/Game/GenericShooter/Addons/Common/Blueprints/Interfaces/BPI_GenericInteractable.Interact`
  (params (Interactor :type "/Game/GenericShooter/Addons/Common/Blueprints/Interfaces/BPI_GenericInteractor Interface"))
  (bind _asactor (cast `Actor` (`KismetSystemLibrary.Conv_InterfaceToObject` Interactor))
    (:`then`
      (bind _returnvalue (`self.GetComponentByClass` _asactor "/Game/GenericShooter/Addons/SlotInventory/Core/BP_SlotInventoryComponent.BP_SlotInventoryComponent_C"))
      (`/Engine/EditorBlueprintResources/StandardMacros.IsValid` _returnvalue
        (:`Is Valid`
          (bind _weaponiteminfo (`self.WeaponItemInfo`)
            (:`then`
              (bind _badded (`/Game/GenericShooter/Addons/SlotInventory/Core/BP_SlotInventoryComponent.AddItem` _returnvalue _weaponiteminfo true))
              (if _badded
                (`self.K2_DestroyActor`)))
            (:`else`
              (`KismetSystemLibrary.PrintString` "ERROR: WeaponProxy interacted with has no item info."))))
        (:`Is Not Valid`
          (`KismetSystemLibrary.PrintString` "ERROR: WeaponProxy interacted with an interactor without a weapon inventory component."))))
    (:`CastFailed`
      (`KismetSystemLibrary.PrintString` "ERROR: WeaponProxy interacted with without an interactor."))))

(fn `CreateItemInfoIfMissing`
  (`self.WeaponItemInfo`
    (:`then`
      (return))
    (:`else`
      (if (or (`KismetSystemLibrary.IsServer`) (`KismetSystemLibrary.IsStandalone`))
        (bind _returnvalue (`|SpawnActorFromClass` (`self.DefaultWeaponItemInfoClass`) (`KismetMathLibrary.MakeTransform` (0.0 0.0 0.0)) "AlwaysSpawn" "OverrideRootScale" null null null))
        (set `self.WeaponItemInfo` _returnvalue)
        (return)
        (else
          (return))))))

(fn `GetDesiredHeldRotation`
  (returns (RelativeHeldRotation :type "Rotator Structure"))
  (return))

(fn `GetInteractionCenterPoint`
  (returns (WorldLocation :type "Vector Structure"))
  (return (0.0 0.0 0.0)))

(fn `GetInteractionText`
  (params (Interactor :type "/Game/GenericShooter/Addons/Common/Blueprints/Interfaces/BPI_GenericInteractor Interface"))
  (returns (Text :type Text))
  (return (`/Game/GenericShooter/Addons/Common/Blueprints/BaseClasses/BP_SlotInventory_ItemInfo_Base.FriendlyItemName` (`self.WeaponItemInfo`))))

(fn `IsFocusable`
  (params (Interactor :type "/Game/GenericShooter/Addons/Common/Blueprints/Interfaces/BPI_GenericInteractor Interface"))
  (returns (bFocusable :type Boolean))
  (return true))

(fn `IsPhysicsPickup`
  (returns (bPickupable :type Boolean) (PickupComponent :type "PrimitiveComponent Object Reference"))
  (return false null))

(fn `ShouldNotInteractOnClients`
  (returns (bShouldNotInteractOnClients :type Boolean))
  (return false))

(fn `ShouldNotSendInteractToServer`
  (returns (bShouldNotSendInteractToServer :type Boolean))
  (return false))

(fn `UserConstructionScript`)