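; Actor component that lets an owner implementing the interactor interface focus, use, and physically carry interactable actors.
; Collider overlaps gather candidates; on tick a line or box trace picks focus by direct hit or fuzzy aim-dot/distance, optionally setting custom depth.
; Pickups follow the owner's target through a physics handle.
; Interact, pickup and release route through server and multicast events, with immediate local execution on remote clients.
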(event Custom|Interact
  (bind _focusedinteractable (Variables|Default|GetFocusedInteractable))
  (bind _focusedinteractable_2 (Variables|Default|GetFocusedInteractable))
  (bind _focusedinteractable_3 (Variables|Default|GetFocusedInteractable))
  (bind _focusedinteractable_4 (Variables|Default|GetFocusedInteractable))
  (bind _returnvalue (Utilities|ToObject(Interface) _focusedinteractable_3))
  (bind _returnvalue_2 (Utilities|ToObject(Interface) _focusedinteractable))
  (bind _returnvalue_3 (Utilities|ToObject(Interface) _focusedinteractable_2))
  (bind _asactor (Utilities|Casting|CastToActor _returnvalue))
  ;[1 1 1] If we are holding something, send network events to release.
  (Utilities|IsValid (Utilities|ToObject(Interface) (Variables|Default|GetHeldPhysicsInteractable))
    (:Is%20Valid
      (Utilities|OwnerasPawnAuthority
        (:Authority
          (CallFunction|MulticastReleaseHeldInteractable false))
        (:Remote
          (CallFunction|ServerReleaseHeldInteractable)
          (CallFunction|ReleaseHeldInteractable))))
    (:Is%20Not%20Valid
      ;[1 1 1] If we can pick something up, send network events to pick it up
      (if (Components|Activation|IsActive)
        (Utilities|IsValid _returnvalue ; Are we looking at an interactable?
          (:Is%20Valid
            (bind _bpickupable (Default|IsPhysicsPickup _focusedinteractable_3))
            (if _bpickupable
              (Utilities|OwnerasPawnAuthority
                (:Authority
                  (CallFunction|MulticastTrytoPickUpInteractable _asactor false))
                (:Remote
                  (CallFunction|ServerTrytoPickUpInteractable _asactor)
                  (CallFunction|TrytoPickUpInteractable)))
              (else
                ;[1 1 1] Handle Interacting
                (Utilities|OwnerasPawnAuthority
                  (:Authority
                    (bind _bshouldnotinteractonclients (Default|ShouldNotInteractonClients _focusedinteractable_4))
                    (if _bshouldnotinteractonclients
                      (Default|Interact (Variables|Default|GetFocusedInteractable) (Variables|Default|GetOwnerAsInteractor))
                      (else
                        (Utilities|DebugPrintNetworkInfo "Calling Multicast Interact" _returnvalue_2
                          (:Out
                            (CallFunction|MulticastInteract (.AsActor (Utilities|Casting|CastToActor _returnvalue_2)) false))))))
                  (:Remote
                    (bind _bshouldnotsendinteracttoserver (Default|ShouldNotSendInteracttoServer _focusedinteractable_4))
                    (if _bshouldnotsendinteracttoserver
                      _
                      (else
                        (Utilities|DebugPrintNetworkInfo "Calling Server Interact" _returnvalue_3
                          (:Out
                            (CallFunction|ServerInteract (.AsActor (Utilities|Casting|CastToActor _returnvalue_3)))))))
                    (Default|Interact (Variables|Default|GetFocusedInteractable) (Variables|Default|GetOwnerAsInteractor)))
                  (:OwnerNotPawn
                    (Default|Interact (Variables|Default|GetFocusedInteractable) (Variables|Default|GetOwnerAsInteractor))))))))))))

(event Custom|MulticastTryToPickUpInteractable
  (params (Interactable :type Actor%20Object%20Reference) (bFromReplication :type Boolean))
  ;[1 1 1] Handles network routing of picking up interactables
  (Utilities|DebugPrintNetworkInfo "Multicast Try Pickup Called" Interactable
    (:Out
      (bind _asinteractable (Utilities|ActorIsValidandIsInteractable Interactable)
        (:Yes
          (bind _blocallycontrolled (Utilities|OwnerasPawnAuthority)
            (:Authority
              (Variables|Default|SetFocusedInteractable _asinteractable :!label _label)
              (CallFunction|TrytoPickUpInteractable))
            (:Remote
              (if (or (and _blocallycontrolled (not bFromReplication)) (not _blocallycontrolled))
                (goto _label)))
            (:OwnerNotPawn
              (goto _label))))))))

(event Custom|ServerTryToPickUpInteractable
  (params (Interactable :type Actor%20Object%20Reference))
  ;[1 1 1] Handles network routing of picking up interactables
  (Utilities|DebugPrintNetworkInfo "Server Try Pickup Called" Interactable
    (:Out
      (Utilities|ActorIsValidandIsInteractable Interactable
        (:Yes
          (CallFunction|MulticastTrytoPickUpInteractable Interactable false))))))

(event Custom|MulticastInteract
  (params (Interactable :type Actor%20Object%20Reference) (bFromReplication :type Boolean))
  ;[1 1 1] Handles network routing of interactions
  (Utilities|DebugPrintNetworkInfo "Multicast Interact called." Interactable
    (:Out
      (bind _asinteractable (Utilities|ActorIsValidandIsInteractable Interactable)
        (:Yes
          (bind _blocallycontrolled (Utilities|OwnerasPawnAuthority)
            (:Authority
              (Default|Interact _asinteractable (Variables|Default|GetOwnerAsInteractor) :!label _label))
            (:Remote
              (if (or (and _blocallycontrolled (not bFromReplication)) (not _blocallycontrolled))
                (goto _label)))
            (:OwnerNotPawn
              (goto _label))))))))

(event Custom|ServerInteract
  (params (Interactable :type Actor%20Object%20Reference))
  (bind _returnvalue (Utilities|String|MakeLiteralString "ERROR: Server received interaction RPC when focused interactable should not send it to the server. Possible desync or cheat."))
  ;[1 1 1] Handles network routing of interactions
  (Utilities|DebugPrintNetworkInfo "Server Interact called." Interactable
    (:Out
      (bind _asinteractable (Utilities|ActorIsValidandIsInteractable Interactable)
        (:Yes
          (bind _bshouldnotsendinteracttoserver (Default|ShouldNotSendInteracttoServer _asinteractable))
          (if _bshouldnotsendinteracttoserver
            (Class|VisualLoggerKismetLibrary|LogText _returnvalue "Blueprint Log")
            (Development|PrintString _returnvalue true true "(R=1.000000,G=0.069580,B=0.000000,A=1.000000)" 5.0)
            (else
              (bind _bshouldnotinteractonclients (Default|ShouldNotInteractonClients _asinteractable))
              (if _bshouldnotinteractonclients
                (Default|Interact _asinteractable (Variables|Default|GetOwnerAsInteractor))
                (else
                  (CallFunction|MulticastInteract Interactable true))))))))))

(event Custom|MulticastReleaseHeldInteractable
  (params (bFromReplication :type Boolean))
  ;[1 1 1] Handles network routing of releasing interactables
  (bind _blocallycontrolled (Utilities|OwnerasPawnAuthority)
    (:Authority
      (CallFunction|ReleaseHeldInteractable :!label _label))
    (:Remote
      (if (or (and _blocallycontrolled (not bFromReplication)) (not _blocallycontrolled))
        (CallFunction|ReleaseHeldInteractable)))
    (:OwnerNotPawn
      (goto _label))))

(event Custom|ServerReleaseHeldInteractable
  ;[1 1 1] Handles network routing of releasing interactables
  (CallFunction|MulticastReleaseHeldInteractable true))

(event EventBeginPlay
  ;[1 1 1] Initialization
  (Utilities|FlowControl|Delay 0.15) ; If we work too fast, sometimes PC doesn't own us or we don't have a viewport for the HUD
  (CallFunction|UpdateOwner)
  (CallFunction|TryAutoSetupInteractionHUDWidget)
  (CallFunction|SetupColliderEvents)
  (CallFunction|SetupPhysicsHandleComponent))

(event EventTick
  (params (DeltaSeconds :type Float%20%28single-precision%29))
  ;[1 1 1] Update interactables on Tick
  (if (Components|Activation|IsActive)
    (CallFunction|UpdateFocusedInteraction)
    (CallFunction|UpdateHeldInteractable)
    (else
      (Utilities|Array|Clear (Variables|Default|GetFocusableInteractables))
      (Variables|Default|SetFocusedInteractable 0)
      (Utilities|IsValid (Utilities|ToObject(Interface) (Variables|Default|GetHeldPhysicsInteractable))
        (:Is%20Valid
          (CallFunction|ReleaseHeldInteractable))))))

(event EventEndPlay
  (params (EndPlayReason :type EEndPlayReason%20Enum :default "Destroyed"))
  ;[1 1 1] Handle destruction
  (bind _autowidgetreference (Variables|Default|GetAutoWidgetReference)
    (:then
      (Widget|RemovefromParent _autowidgetreference)
      (Variables|Default|SetAutoWidgetReference 0)
      (Components|Activation|SetActive false false))
    (:else)))

(fn OnColliderBeginOverlap
  (params (OverlappedComponent :type Primitive%20Component%20Object%20Reference) (OtherActor :type Actor%20Object%20Reference) (OtherComponent :type Primitive%20Component%20Object%20Reference) (OtherBodyIndex :type Integer) (bFromSweep :type Boolean) (SweepResult :type Hit%20Result%20Structure%20%28by%20ref%29))
  (Utilities|IsValid OtherActor ; Used for checking if actor is pending kill
    (:Is%20Valid
      (bind _asbpi_generic_interactable (Utilities|Casting|CastToBPI_GenericInteractable OtherActor)
        (:then
          (Utilities|Array|AddUnique (Variables|Default|GetFocusableInteractables) _asbpi_generic_interactable))
        (:CastFailed
          _)))
    (:Is%20Not%20Valid
      _))
  (return))

(fn OnColliderEndOverlap
  (params (OverlappedComponent :type Primitive%20Component%20Object%20Reference) (OtherActor :type Actor%20Object%20Reference) (OtherComponent :type Primitive%20Component%20Object%20Reference) (OtherBodyIndex :type Integer))
  (bind _asbpi_generic_interactable (Utilities|Casting|CastToBPI_GenericInteractable OtherActor)
    (:then
      (bind _returnvalue (Utilities|Array|RemoveItem (Variables|Default|GetFocusableInteractables) _asbpi_generic_interactable))
      (if _returnvalue
        (Default|SetFocused _asbpi_generic_interactable 0 false)))
    (:CastFailed
      _))
  (return))

(fn SetupColliderEvents
  (bind _collider (Class|BPIGenericInteractor|GetInteractionCollider(Message) (Components|GetOwner)))
  (bind _output_get (Variables|Default|SetOwnerCollider _collider))
  (Utilities|IsValid _output_get
    (:Is%20Valid
      _)
    (:Is%20Not%20Valid
      ;[1 1 1] No collider returned? Interface possibly not implemented, try to find collider ourselves
      (if (Variables|Config|GetbTryToFindRootPrimitiveComponent)
        (bind _asactor (Utilities|Casting|CastToActor (Variables|Default|GetOwnerAsInteractor))
          (:then
            (bind _asprimitive_component (Utilities|Casting|CastToPrimitiveComponent (VehicleSound|GetRootComponent _asactor))
              (:then
                (Variables|Default|SetOwnerCollider _asprimitive_component))
              (:CastFailed
                (return))))
          (:CastFailed
            (return)))
        (else
          (return)))))
  (Utilities|FlowControl|Sequence
    (:then_0
      (Collision|BindEventtoOnComponentBeginOverlap (Variables|Default|GetOwnerCollider) (EventDispatchers|CreateEvent :!event OnColliderBeginOverlap)))
    (:then_1
      (Collision|BindEventtoOnComponentEndOverlap (Variables|Default|GetOwnerCollider) (EventDispatchers|CreateEvent :!event OnColliderEndOverlap))
      (return))))

(fn UpdateFocusedInteraction
  (bind _lasttraceinfo (Variables|Default|GetLastTraceInfo))
  (bind _lasttraceinfo_2 (Variables|Default|GetLastTraceInfo))
  (bind (_bblockinghit _binitialoverlap _time _distance _location _impactpoint _normal _impactnormal _physmat _hitactor) (Collision|BreakHitResult _lasttraceinfo))
  (bind (_bblockinghit_2 _binitialoverlap_2 _time_2 _distance_2 _location_2 _impactpoint_2 _normal_2 _impactnormal_2 _physmat_2 _hitactor_2 _hitcomponent _hitbonename _hititem _faceindex _tracestart _traceend) (Collision|BreakHitResult _lasttraceinfo_2))
  ;[1 1 1] If holding something, treat it as best interactable.
  (bind _asactor (Utilities|Casting|CastToActor (Utilities|ToObject(Interface) (Variables|Default|GetHeldPhysicsInteractable)))
    (:then
      (LocalVariables|SetBestInteractable _asactor)
      ;[1 1 1] If Focused interactable has changed...
      (if (!= (LocalVariables|GetBestInteractable) (Utilities|ToObject(Interface) (Variables|Default|GetFocusedInteractable))) :!label _label
        ;[1 1 1] Clear custom depth on old interactable
        (if (Variables|Config|Visuals|GetbSetRenderCustomDepthOnFocus)
          (CallFunction|SetRenderCustomDepthonInteractable false (Variables|Default|GetFocusedInteractable)))
        ;[1 1 1] Unfocusing old and focusing the new interactable
        (Utilities|IsValid (Utilities|ToObject(Interface) (Variables|Default|GetFocusedInteractable))
          (:Is%20Valid
            (Class|BPIGenericInteractable|SetFocused(Message) (Utilities|ToObject(Interface) (Variables|Default|GetFocusedInteractable)) (Variables|Default|GetOwnerAsInteractor) false))
          (:Is%20Not%20Valid
            _))
        (bind _output_get (Variables|Default|SetFocusedInteractable (.AsBPI%20Generic%20Interactable (Utilities|Casting|CastToBPI_GenericInteractable (LocalVariables|GetBestInteractable)))))
        (if (.bSuccess (Utilities|Casting|CastToBPI_GenericInteractable (LocalVariables|GetBestInteractable)))
          (Default|SetFocused _output_get (Variables|Default|GetOwnerAsInteractor) true)
          ;[1 1 1] If we're responsible for enabling custom depth, enable it now for new focused interactable
          (if (Variables|Config|Visuals|GetbSetRenderCustomDepthOnFocus)
            (CallFunction|SetRenderCustomDepthonInteractable true (Variables|Default|GetFocusedInteractable))
            (return)
            (else
              (return)))
          (else
            (return)))
        (else
          (return))))
    (:CastFailed
      (if (CallFunction|ShouldLineTrace)
        (CallFunction|PerformLineTrace)
        (bind _array_element (Utilities|Array|ForEachLoopwithBreak (Variables|Default|GetFocusableInteractables) :!label _label_2)
          (:LoopBody
            ;[1 1 1] Do a pruning of any possibly bad focusable interactables from our focusable list
            (bind _asactor_2 (Utilities|Casting|CastToActor _array_element))
            (LocalVariables|SetTestInteractable _asactor_2)
            (LocalVariables|GetTestInteractable
              (:then
                (if (Utilities|Array|ContainsItem (Class|Actor|GetOverlappingComponents (LocalVariables|GetTestInteractable)) (Variables|Default|GetOwnerCollider))
                  ;[1 1 1] Make sure this interactable is even focusable first
                  (bind _bfocusable (Class|BPIGenericInteractable|IsFocusable(Message) (LocalVariables|GetTestInteractable) (Variables|Default|GetOwnerAsInteractor)))
                  (if _bfocusable
                    ;[1 1 1] Grab possibly overriden world location for interaction tests
                    (bind _returnvalue (CallFunction|GetInteractableWorldLocation (LocalVariables|GetTestInteractable)))
                    (LocalVariables|SetTestInteractionCenterPoint _returnvalue)
                    ;[1 1 1] Are we directly looking at an interactable? If so, flag this as best and move on
                    (if (and _bblockinghit (== _hitactor (LocalVariables|GetTestInteractable)))
                      (LocalVariables|SetBestInteractable (LocalVariables|GetTestInteractable))
                      (goto _label_2 Break)
                      (else
                        ;[1 1 1] Calculate Dot Product between aim point and interactable
                        (bind _output_get_2 (LocalVariables|SetTestDotProduct (|(Dot((Normalize(({10D11FF9-4AE0-E315-5028-ED97DFC6BEC2}-TraceStart))),(Normalize((EndPoint-TraceStart))))) _tracestart (Math|Vector|SelectVector _impactpoint_2 _traceend _bblockinghit_2))))
                        (if (>= _output_get_2 (Variables|Config|GetMinimumDotProduct))
                          ;[1 1 1] Stop testing here if exact aim is required
                          (if (Variables|Config|GetbAllowFuzzyFocus)
                            ;[0.7585 1 0.7438] Prioritize based on Distance or Dot Product?
                            (if (Variables|Config|GetbPrioritizeBasedOnDistance)
                              ;[1 1 1] Prioritize interactables based on distance
                              (Class|BPIGenericInteractable|SetInteractionDebugString(Message) (LocalVariables|GetTestInteractable) (Variables|Default|GetOwnerAsInteractor) (Utilities|String|ToString(Float) (Math|Vector|VectorLengthSquared (- (LocalVariables|GetTestInteractionCenterPoint) (.ImpactPoint (Collision|BreakHitResult (Variables|Default|GetLastTraceInfo)))))))
                              (if (< (Math|Vector|VectorLengthSquared (- (LocalVariables|GetTestInteractionCenterPoint) (.ImpactPoint (Collision|BreakHitResult (Variables|Default|GetLastTraceInfo))))) (LocalVariables|GetBestDistance))
                                (LocalVariables|SetBestInteractable (LocalVariables|GetTestInteractable))
                                (LocalVariables|SetBestDistance (Math|Vector|VectorLengthSquared (- (LocalVariables|GetTestInteractionCenterPoint) (.ImpactPoint (Collision|BreakHitResult (Variables|Default|GetLastTraceInfo)))))))
                              (else
                                ;[1 1 1] Prioritize based on Dot Product
                                (Class|BPIGenericInteractable|SetInteractionDebugString(Message) (LocalVariables|GetTestInteractable) (Variables|Default|GetOwnerAsInteractor) (Utilities|String|ToString(Float) (LocalVariables|GetTestDotProduct)))
                                (if (> (LocalVariables|GetTestDotProduct) (LocalVariables|GetBestDotProduct))
                                  (LocalVariables|SetBestInteractable (LocalVariables|GetTestInteractable))
                                  (LocalVariables|SetBestDotProduct (LocalVariables|GetTestDotProduct))))))))))
                  (else
                    (Utilities|Array|Add (LocalVariables|GetInteractablesToRemove) _array_element :!label _label_3))))
              (:else
                (goto _label_3))))
          (:Completed
            ;[1 1 1] Remove interactables that are not valid but not caught by OnColliderEndOverlap
            (for _array_element_2 (LocalVariables|GetInteractablesToRemove)
              (Utilities|Array|RemoveItem (Variables|Default|GetFocusableInteractables) _array_element_2))
            (goto _label)))
        (else
          ;[1 1 1] If no valid focusable interactables are in range, make sure we clear focus on anything that we might have beenf ocusing on
          (Utilities|IsValid (Utilities|ToObject(Interface) (Variables|Default|GetFocusedInteractable))
            (:Is%20Valid
              (Default|SetFocused (Variables|Default|GetFocusedInteractable) (Variables|Default|GetOwnerAsInteractor) false)
              ;;[0.25 0.25 0.25] Clear custom depth on old interactable
              (if (Variables|Config|Visuals|GetbSetRenderCustomDepthOnFocus)
                (CallFunction|SetRenderCustomDepthonInteractable false (Variables|Default|GetFocusedInteractable))))
            (:Is%20Not%20Valid
              _))
          (Variables|Default|SetFocusedInteractable 0)
          (return))))))

(fn PerformLineTrace
  (bind (_startpoint _aimdirection) (CallFunction|GetTraceInfofromOwner))
  (bind _btracecomplex (Variables|Config|GetbTraceComplex))
  (bind _tracedebugdraw (Variables|Config|GetTraceDebugDraw))
  (bind _bignoreself (Variables|Config|GetbIgnoreSelf))
  (bind _tracechannel (Variables|Config|GetTraceChannel))
  ;[1 1 1] Grabs trace info from our owner, generally our aim direction.
  (LocalVariables|SetStartPoint _startpoint)
  (LocalVariables|SetEndPoint (+ (LocalVariables|GetStartPoint) (* (Math|Vector|Normalize _aimdirection) (Variables|Config|GetRange))))
  (bind _actorstoignore (Default|GetInteractionIgnoreList (Variables|Default|GetOwnerAsInteractor)))
  (if (not (Variables|Config|BoxTracing|GetbUseBoxInsteadOfLineTracing))
    (bind _outhit (Collision|LineTraceByChannel (LocalVariables|GetStartPoint) (LocalVariables|GetEndPoint) _tracechannel _btracecomplex _actorstoignore _tracedebugdraw _bignoreself))
    (Variables|Default|SetLastTraceInfo _outhit)
    (return)
    (else
      (bind _outhit_2 (Collision|BoxTraceByChannel (LocalVariables|GetStartPoint) (LocalVariables|GetEndPoint) (Variables|Config|BoxTracing|GetBoxTraceHalfSize) "0, 0, 0" _tracechannel _btracecomplex _actorstoignore _tracedebugdraw _bignoreself))
      (Variables|Default|SetLastTraceInfo _outhit_2)
      (return))))

(fn GetTraceInfofromOwner
  (bind _busecameramanagerwhentraceinfonotimplemented (Variables|Config|GetbUseCameraManagerWhenTraceInfoNotImplemented))
  (bind (_startpoint _aimdirection) (Default|GetInteractionTraceLine (Variables|Default|GetOwnerAsInteractor)))
  (if (and (Math|Vector|Equal(Vector) _startpoint _aimdirection 0.0001) (Math|Vector|Equal(Vector) _aimdirection "0, 0, 0" 0.0001))
    (bind _aspawn (Utilities|Casting|CastToPawn (Variables|Default|GetOwnerAsInteractor))
      (:then
        (bind _asplayer_controller (Utilities|Casting|CastToPlayerController (Pawn|GetController _aspawn))
          (:then
            (return (Math|Vector|SelectVector (Camera|GetCameraLocation (Variables|/Script/Engine.PlayerController|GetPlayerCameraManager _asplayer_controller)) (.OutLocation (Actor|GetActorEyesViewPoint (Pawn|GetViewTarget _asplayer_controller))) _busecameramanagerwhentraceinfonotimplemented) (Math|Rotator|GetRotationXVector (Math|Rotator|SelectRotator (Camera|GetCameraRotation (Variables|/Script/Engine.PlayerController|GetPlayerCameraManager _asplayer_controller)) (.OutRotation (Actor|GetActorEyesViewPoint (Pawn|GetViewTarget _asplayer_controller))) _busecameramanagerwhentraceinfonotimplemented))))
          (:CastFailed
            _)))
      (:CastFailed
        _))
    (return "0, 0, 0" "0, 0, 0")
    (else
      (return _startpoint _aimdirection))))

(fn SetRenderCustomDepthonInteractable
  (params (bRenderCustomDepth :type Boolean) (Interactable :type BPI%20Generic%20Interactable%20Interface))
  (if (CallFunction|IsOwnerPawnandLocallyControlled)
    (bind _asactor (Utilities|Casting|CastToActor Interactable)
      (:then
        (Utilities|IsValid _asactor ; IsPendingKill?
          (:Is%20Valid
            (Rendering|SetRenderCustomDepth (Actor|GetComponentsByClass _asactor "/Script/Engine.PrimitiveComponent") bRenderCustomDepth)
            (Rendering|SetCustomDepthStencilValue (Actor|GetComponentsByClass _asactor "/Script/Engine.PrimitiveComponent") (Variables|Config|Visuals|GetRenderCustomDepthStencilValue))
            (return))
          (:Is%20Not%20Valid
            _)))
      (:CastFailed
        _)))
  (return))

(fn TryAutoSetupInteractionHUDWidget
  ;[1 1 1] If we shouldn't be creating this widget, simply return early.
  (if (Variables|Config|UI|GetbShouldAutoCreateInteractWidget)
    ;[1 1 1] Only add UI if we are a locally controlled player controller.
    (bind _aspawn (Utilities|Casting|CastToPawn (Variables|Default|GetOwnerAsInteractor))
      (:then
        (if (Pawn|IsLocallyControlled _aspawn)
          (bind _asplayer_controller (Utilities|Casting|CastToPlayerController (Pawn|GetController _aspawn))
            (:then
              (bind _returnvalue (UserInterface|CreateWidget "/Game/GenericShooter/Addons/Interaction/Core/WBP_GenericInteractionWidget.WBP_GenericInteractionWidget_C" _asplayer_controller (Variables|Default|GetOwnerAsInteractor)))
              (bind _output_get (Variables|Default|SetAutoWidgetReference _returnvalue))
              (UserInterface|Viewport|AddtoPlayerScreen _output_get (Variables|Config|UI|GetWidgetZOrder))
              (return))
            (:CastFailed
              _))))
      (:CastFailed
        _))
    (return)
    (else
      (return))))

(fn SetupPhysicsHandleComponent
  ;[1 1 1] If owner gives us a physics handle, lets just go ahead and use that.
  (bind _physicshandlecomponent (Class|BPIGenericInteractor|GetPhysicsHandle(Message) (Components|GetOwner)))
  (bind _output_get (Variables|Default|SetPhysicsHandleComponent _physicshandlecomponent))
  (Utilities|IsValid _output_get
    (:Is%20Valid
      (return))
    (:Is%20Not%20Valid
      ;[1 1 1] If it doesn't we'll try finding it.
      (if (Variables|Config|GetbTryToFindPhysicsHandleComponent)
        (Variables|Default|SetPhysicsHandleComponent (Actor|GetComponentbyClass (Components|GetOwner) "/Script/Engine.PhysicsHandleComponent"))
        (return)
        (else
          (return))))))

(fn ReleaseHeldInteractable
  (Utilities|IsValid (Utilities|ToObject(Interface) (Variables|Default|GetHeldPhysicsInteractable))
    (:Is%20Valid
      (Physics|Components|PhysicsHandle|ReleaseComponent (Variables|Default|GetPhysicsHandleComponent))
      (Default|OnPhysicsRelease (Variables|Default|GetHeldPhysicsInteractable) (Variables|Default|GetOwnerAsInteractor) (Variables|Default|GetPhysicsHandleComponent))
      (Variables|Default|SetPickedUpComponent 0)
      (Variables|Default|SetHeldPhysicsInteractable 0)
      (return true))
    (:Is%20Not%20Valid
      (return false))))

(fn TrytoPickUpInteractable
  ;[1 1 1] If we have no physics handle, return as we won't ever be able to pick up anything.
  (Utilities|IsValid (Variables|Default|GetPhysicsHandleComponent)
    (:Is%20Valid
      ;[1 1 1] If focused object isn't a physical pickup, do nothing
      (bind (_bpickupable _pickupcomponent) (Default|IsPhysicsPickup (Variables|Default|GetFocusedInteractable)))
      (if (and _bpickupable (Utilities|IsValid _pickupcomponent))
        (bind _output_get (Variables|Default|SetHeldPhysicsInteractable (Variables|Default|GetFocusedInteractable)))
        (bind _output_get_2 (Variables|Default|SetPickedUpComponent _pickupcomponent))
        (bind _relativeheldrotation (Default|GetDesiredHeldRotation _output_get))
        (Variables|Default|SetDesiredHeldRotationOffset _relativeheldrotation)
        (bind (_handlelocation _handlerotation) (Default|GetPhysicsHandleTargetLocationandRotation (Variables|Default|GetOwnerAsInteractor)))
        (Transformation|SetWorldLocationAndRotation (Variables|Default|GetPickedUpComponent) _handlelocation (Math|Rotator|CombineRotators (Variables|Default|GetDesiredHeldRotationOffset) _handlerotation) false true) ; Align Object before grabbing
        (Physics|Components|PhysicsHandle|GrabComponentatLocationwithRotation (Variables|Default|GetPhysicsHandleComponent) (Variables|Default|GetPickedUpComponent) "None" (Transformation|GetWorldLocation _output_get_2) (Math|Rotator|CombineRotators (Variables|Default|GetDesiredHeldRotationOffset) _handlerotation))
        (Default|OnPhysicsPickup (Variables|Default|GetFocusedInteractable) (Variables|Default|GetOwnerAsInteractor) (Variables|Default|GetPhysicsHandleComponent))
        (return true)
        (else
          (return false))))
    (:Is%20Not%20Valid
      (return false))))

(fn UpdateHeldInteractable
  ;[1 1 1] If our physics handle or picked up component is null, there is no point in updating
  (Variables|Default|GetPhysicsHandleComponent
    (:then
      (Variables|Default|GetPickedUpComponent
        (:then
          (bind (_handlelocation _handlerotation) (Default|GetPhysicsHandleTargetLocationandRotation (Variables|Default|GetOwnerAsInteractor)))
          (if (Math|Vector|NotEqual(Vector) _handlelocation "0, 0, 0" 0.0001)
            (Class|PhysicsHandleComponent|SetTargetLocationandRotation (Variables|Default|GetPhysicsHandleComponent) _handlelocation (Math|Rotator|CombineRotators (Variables|Default|GetDesiredHeldRotationOffset) _handlerotation))
            (else
              (Development|PrintString "Error: Interaction Component picked up physics object but owner does not have GetPhysicsHandleTargetLocation implemented!" true true "(R=1.000000,G=0.000000,B=0.039114,A=1.000000)" 1.0)))
          (return))
        (:else
          _)))
    (:else
      _))
  (return))

(fn UpdateOwner
  (bind _returnvalue (Components|GetOwner))
  (if (Utilities|DoesObjectImplementInterface _returnvalue "/Game/GenericShooter/Addons/Common/Blueprints/Interfaces/BPI_GenericInteractor.BPI_GenericInteractor_C")
    (bind _asbpi_generic_interactor (Utilities|Casting|CastToBPI_GenericInteractor _returnvalue)
      (:then
        (Variables|Default|SetOwnerAsInteractor _asbpi_generic_interactor)
        (return))
      (:CastFailed
        _))
    (else
      (Class|VisualLoggerKismetLibrary|LogText "Interaction Component assigned to an actor that does not implement the Interactor interface!" "Blueprint Log")))
  (return))

(fn IsOwnerPawnandLocallyControlled
  (bind _aspawn (Utilities|Casting|CastToPawn (Utilities|ToObject(Interface) (Variables|Default|GetOwnerAsInteractor)))
    (:then
      (if (Pawn|IsLocallyControlled _aspawn)
        (return (Pawn|IsLocallyControlled _aspawn))
        (else
          _)))
    (:CastFailed
      _))
  (return false))

(fn GetInteractableWorldLocation
  (params (Interactable :type Actor%20Object%20Reference))
  (bind _worldlocation (Default|GetInteractionCenterPoint (.AsBPI%20Generic%20Interactable (Utilities|Casting|CastToBPI_GenericInteractable Interactable))))
  (return (Math|Vector|SelectVector (Transformation|GetActorLocation Interactable) _worldlocation (Math|Vector|Equal(Vector) _worldlocation "0, 0, 0" 0.0001))))

(fn ShouldLineTrace
  (return (or (!= (Utilities|Array|Length (Variables|Default|GetFocusableInteractables)) 0) (Variables|Config|GetbPerformLineTraceEvenWithoutFocusableInteractables))))