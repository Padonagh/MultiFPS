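; Component that stores a team member's team number and relays team change requests in the GenericShooter TeamManager addon.
; ServerRequestTeamChange forwards the member object and desired team to the BP_TeamManagerComponent on the GameState.
; SetTeamNum writes only on the server, and the TeamNum RepNotify calls OnTeamNumChanged with the new value.
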(event `ServerRequestTeamChange`
  (params (TeamMemberObject :type "Object Object Reference") (DesiredTeam :type Integer))
  (`/Game/GenericShooter/Addons/TeamManager/Core/BP_TeamManagerComponent.RequestTeamChange` (`Actor.GetComponentByClass` (`GameplayStatics.GetGameState`) "/Game/GenericShooter/Addons/TeamManager/Core/BP_TeamManagerComponent.BP_TeamManagerComponent_C") TeamMemberObject DesiredTeam))

(fn `GetTeamNum`
  (returns (TeamNum :type Byte))
  (return (`self.TeamNum`)))

(fn `OnRep_TeamNum`
  (`self.OnTeamNumChanged` (`self.TeamNum`))
  (return))

(fn `SetTeamNum`
  (params (TeamNum :type Byte))
  (if (`KismetSystemLibrary.IsServer`)
    (set `self.TeamNum` TeamNum)
    (return)
    (else
      (return))))