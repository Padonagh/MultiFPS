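; Blueprint function library that resolves a hit bone to its hit zone data.
; GetHitzoneInfoForBone looks up the bone's zone name in a bone-to-zone data table, then joins it to a given prefix with an underscore.
; That prefixed name is the row key into the hit zone table, returning the row and name, or None and a false found flag if either lookup fails.
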(fn `GetHitzoneInfoForBone`
  (params (HitzonePrefix :type String :default "Default") (BoneName :type Name) (BoneHitzoneLookupTable :type "DataTable Object Reference") (HitzoneTable :type "DataTable Object Reference"))
  (returns (HitZoneName :type Name) (HitZoneInfo :type "/Game/GenericShooter/Addons/Common/Blueprints/HitZones/FHitZoneInfo Structure") (bFoundHitZone :type Boolean))
  (bind _returnvalue (`|GetDataTableRow` BoneHitzoneLookupTable BoneName)
    (:`then`
      (bind _returnvalue_2 (`KismetStringLibrary.Conv_StringToName` (`KismetStringLibrary.Concat_StrStr` (`local.HitzonePrefix`) "_" (`KismetStringLibrary.Conv_NameToString` (`.HitZoneName_2_862CA15E4A622FA929BC23A18E35F97E` (break `/Game/GenericShooter/Addons/Common/Blueprints/HitZones/FBoneHitZoneLookup` _returnvalue))))))
      (bind _returnvalue_3 (`|GetDataTableRow` (`local.HitzoneTable`) _returnvalue_2)
        (:`then`
          (return _returnvalue_2 _returnvalue_3 true))
        (:`RowNotFound`
          (return "None" (struct) false))))
    (:`RowNotFound`
      (return "None" (struct) false))))