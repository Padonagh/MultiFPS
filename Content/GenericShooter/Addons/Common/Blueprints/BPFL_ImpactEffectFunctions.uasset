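; Blueprint function library that spawns surface-dependent impact particles, sounds and decals from hit results.
; Effects are looked up by physical surface in an impact class's default map, with default-surface fallback and error logs, or in a data table by "Category_Surface" row name.
; Both paths feed SpawnPhysicalMaterialEffect, which adds a randomly rolled, attached decal on blocking hits and otherwise places effects at trace start along the trace direction.
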(fn `SpawnImpactEffectsFromImpactClass`
  (params (ImpactClass :type "/Game/GenericShooter/Addons/Common/Blueprints/BaseClasses/BP_ImpactEffect_Base Class Reference") (HitInfo :type "HitResult Structure") (ActorResponsible :type "Actor Object Reference") (VolumeScale :type "Float (double-precision)" :default 1.0))
  (bind (_bblockinghit _binitialoverlap _time _distance _location _impactpoint _normal _impactnormal _physmat) (`GameplayStatics.BreakHitResult` HitInfo))
  (bind _surfacemap (defaults `Object` ImpactClass))
  (bind _actorresponsible (`local.ActorResponsible`))
  (bind _returnvalue (select `bool` (`KismetSystemLibrary.IsValid` _physmat) :`false` "SurfaceType_Default" :`true` (`PhysicalMaterial.SurfaceType` _physmat)))
  (bind _returnvalue_2 (select `bool` (`BlueprintMapLibrary.Map_Contains` _surfacemap _returnvalue) :`false` "SurfaceType_Default" :`true` _returnvalue))
  (bind (_value _returnvalue_3) (`BlueprintMapLibrary.Map_Find` _surfacemap _returnvalue_2))
  (if (`KismetSystemLibrary.IsValidClass` ImpactClass)
    (if _returnvalue_3
      (`self.SpawnPhysicalMaterialEffect` _value (`local.HitInfo`) _actorresponsible 10.0 (`local.VolumeScale`) _actorresponsible)
      (else
        (`VisualLoggerKismetLibrary.LogText` (`KismetTextLibrary.Conv_TextToString` (`|FormatText` "ERROR: {Me}: Tried spawning impact effect but did not have impact visuals defined for surface type {SurfaceType}." (`KismetTextLibrary.Conv_StringToText` (`KismetSystemLibrary.GetObjectName` (`local.ActorResponsible`))) (`KismetTextLibrary.Conv_NameToText` (`|GetEnumeratorName` _returnvalue_2)))))
        (return)))
    (else
      (`VisualLoggerKismetLibrary.LogLocation` _impactpoint (`KismetTextLibrary.Conv_TextToString` (`|FormatText` "ERROR: {Me}: Tried spawning impact effect but did not have a valid impact class set." (`KismetTextLibrary.Conv_StringToText` (`KismetSystemLibrary.GetObjectName` (`local.ActorResponsible`))))) (struct :`R` 1.0 :`B` 0.026156 :`A` 1.0)))))

(fn `SpawnPhysicalMaterialEffect`
  (params (EffectInfo :type "/Game/GenericShooter/Addons/Common/Blueprints/FPhysicalMaterialEffectInfo Structure") (HitInfo :type "HitResult Structure") (ActorResponsible :type "Actor Object Reference") (DecalThickness :type "Float (double-precision)" :default 10.0) (VolumeScale :type "Float (double-precision)" :default 1.0))
  (locals (NormalRotation :type "Rotator Structure") (DecalRotation :type "Rotator Structure") (SpawnLocation :type "Vector Structure"))
  (bind (_effect _sound _decalmaterial _decalsize _decallifetime) (break `/Game/GenericShooter/Addons/Common/Blueprints/FPhysicalMaterialEffectInfo` (`local.EffectInfo`)))
  (bind (_bblockinghit _binitialoverlap _time _distance _location _impactpoint _normal _impactnormal _physmat _hitactor _hitcomponent _hitbonename _hititem _faceindex _tracestart _traceend) (`GameplayStatics.BreakHitResult` (`local.HitInfo`)))
  (bind (_bblockinghit_2 _binitialoverlap_2 _time_2 _distance_2 _location_2 _impactpoint_2 _normal_2 _impactnormal_2 _physmat_2 _hitactor_2 _hitcomponent_2 _hitbonename_2) (`GameplayStatics.BreakHitResult` (`local.HitInfo`)))
  ;[1 1 1] Calculate Spawn location, impact normal based rotation, and a random rotation to use for decals
  (set `local.SpawnLocation` (`KismetMathLibrary.SelectVector` _impactpoint _tracestart _bblockinghit))
  (set `local.NormalRotation` (`KismetMathLibrary.SelectRotator` (`/Game/GenericShooter/Addons/Common/BPFL_CommonMath.VectorToRotatorWithTolerance` _impactnormal (`local.ActorResponsible`)) (`KismetMathLibrary.Conv_VectorToRotator` (`KismetMathLibrary.Normal` (- _traceend _tracestart))) _bblockinghit))
  (set `local.DecalRotation` (`KismetMathLibrary.ComposeRotators` (`KismetMathLibrary.MakeRotator` (`KismetMathLibrary.RandomFloatInRange` 0.0 360.0)) (`KismetMathLibrary.MakeRotFromX` _impactnormal)))
  (`|ExecutionSequence`
    (:`then_0`
      ;[1 1 1] Spawn Emitter and Sound
      (`GameplayStatics.SpawnEmitterAtLocation` (`local.ActorResponsible`) _effect (`local.SpawnLocation`) (`local.NormalRotation`)))
    (:`then_1`
      (`GameplayStatics.SpawnSoundAtLocation` (`local.ActorResponsible`) _sound (`local.SpawnLocation`) (struct) (`local.VolumeScale`)))
    (:`then_2`
      ;[1 1 1] Spawn Decal if this is a blocking hit
      (if _bblockinghit_2
        (`GameplayStatics.SpawnDecalAttached` _decalmaterial (`KismetMathLibrary.MakeVector` (`local.DecalThickness`) _decalsize _decalsize) _hitcomponent_2 _hitbonename_2 (+ (`local.SpawnLocation`) (* _impactnormal_2 5.0)) (`local.DecalRotation`) "KeepWorldPosition" _decallifetime)))
    (:`then_3`
      (return))))

(fn `SpawnPhysicalMaterialEffectFromDataTable`
  (params (EffectCategoryKey :type Name) (DataTable :type "DataTable Object Reference") (HitInfo :type "HitResult Structure") (ActorResponsible :type "Actor Object Reference") (VolumeScale :type "Float (double-precision)" :default 1.0))
  (locals (KeyName :type Name))
  (bind (_bblockinghit _binitialoverlap _time _distance _location _impactpoint _normal _impactnormal _physmat) (`GameplayStatics.BreakHitResult` HitInfo))
  (bind _returnvalue (`KismetStringLibrary.Conv_NameToString` EffectCategoryKey))
  (bind _actorresponsible (`local.ActorResponsible`))
  ;[1 1 1] Build effect key name and pull it from the data table
  (`/Engine/EditorBlueprintResources/StandardMacros.IsValid` _physmat
    (:`Is Valid`
      (set `local.KeyName` (`KismetStringLibrary.Conv_StringToName` (`KismetStringLibrary.Concat_StrStr` _returnvalue "_" (`|GetEnumeratorNameAsString` (`PhysicalMaterial.SurfaceType` _physmat))))))
    (:`Is Not Valid`
      (set `local.KeyName` (`KismetStringLibrary.Conv_StringToName` (`KismetStringLibrary.Concat_StrStr` _returnvalue "_" "Default")))))
  (bind _returnvalue_2 (`|GetDataTableRow` (`local.DataTable`) (`local.KeyName`))
    (:`then`
      (`self.SpawnPhysicalMaterialEffect` _returnvalue_2 (`local.HitInfo`) _actorresponsible 10.0 (`local.VolumeScale`) _actorresponsible)
      (return))
    (:`RowNotFound`
      (return))))