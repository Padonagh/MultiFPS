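; Player start for the generic shooter that filters spawning by team and labels itself with its team number or "Any" via a text render set in construction.
; In team games, per the game state's team manager component, it accepts controllers whose player state team matches, or anyone if flagged AnyTeam.
; Otherwise it is valid unless disabled for non-team games.
; A separate check reports pawns overlapping its PawnCheckRadius component.
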(fn `IsPawnAtSpawn`
  (returns (bYes :type Boolean))
  (bind _pawncheckradius (`self.PawnCheckRadius`))
  (bind (_outactors _returnvalue) (`KismetSystemLibrary.ComponentOverlapActors` _pawncheckradius (`SceneComponent.K2_GetComponentToWorld` _pawncheckradius) (`|MakeArray` "ObjectTypeQuery3" :!type "EObjectTypeQuery Enum") "/Script/Engine.Pawn"))
  (return _returnvalue))

(fn `IsValidSpawnPointForController`
  (params (Controller :type "Controller Object Reference"))
  (returns (bIsValid :type Boolean))
  (bind _returnvalue (`self.GetComponentByClass` (`GameplayStatics.GetGameState`) "/Game/GenericShooter/Addons/TeamManager/Core/BP_TeamManagerComponent.BP_TeamManagerComponent_C"))
  (`/Engine/EditorBlueprintResources/StandardMacros.IsValid` _returnvalue
    (:`Is Valid`
      (if (`/Game/GenericShooter/Addons/TeamManager/Core/BP_TeamManagerComponent.IsTeamGame` _returnvalue)
        (bind _teamnum (message `/Game/GenericShooter/Addons/Common/Blueprints/Interfaces/BPI_TeamMember.GetTeamNum` (`Controller.PlayerState` Controller)))
        (return (or (== _teamnum (`self.TeamNum`)) (`self.bAnyTeam`)))
        (else
          _)))
    (:`Is Not Valid`
      _))
  (return (not (`self.bDisabledInNoTeamGames`))))

(fn `UserConstructionScript`
  (`TextRenderComponent.K2_SetText` (`self.TextRender`) (select `bool` (`self.bAnyTeam`) :`false` (`KismetTextLibrary.Conv_ByteToText` (`self.TeamNum`)) :`true` "Any")))