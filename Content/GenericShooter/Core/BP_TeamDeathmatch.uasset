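; BP_TeamDeathmatch is the team deathmatch game mode, configuring a match from the game mode options string.
; SetGameOptions first seeds the game state's BP_TeamManagerComponent with the default team count, then lets the game state configure itself from the same options.
; It then parses kill limit, current max players and a LAN-only flag, using existing values as defaults for the two numeric settings, and returns true.
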(fn `SetGameOptions`
  (params (Options :type String))
  (returns (bSet :type Boolean))
  (`|ExecutionSequence`
    (:`then_0`
      ;[1 1 1] Set Number of teams to default team count, then give game state a chance to configure itself using game mode option string
      (`/Game/GenericShooter/Addons/TeamManager/Core/BP_TeamManagerComponent.SetNumTeams` (`self.GetComponentByClass` (`GameplayStatics.GetGameState`) "/Game/GenericShooter/Addons/TeamManager/Core/BP_TeamManagerComponent.BP_TeamManagerComponent_C") (`self.DefaultNumTeams`))
      (`/Game/GenericShooter/Core/BPFL_GenericShooterExampleLogic.ExampleSetGameStateOptions` (`local.Options`)))
    (:`then_1`
      ;[1 1 1] Kill Limit
      (set `self.KillLimit` (`GameplayStatics.GetIntOption` (`local.Options`) (`self.KillLimitKey`) (`self.KillLimit`))))
    (:`then_2`
      ;[1 1 1] Set Current Max Players
      (set `self.CurrentMaxPlayers` (`GameplayStatics.GetIntOption` (`local.Options`) (`self.CurrentMaxPlayersKey`) (`self.MaxPlayers`))))
    (:`then_3`
      ;[1 1 1] Set Lan Only Desired
      (set `self.bLanOnlyDesired` (`GameplayStatics.HasOption` (`local.Options`) (`self.LanOnlyKey`))))
    (:`then_4`
      (return true))))

(fn `UserConstructionScript`
  (`parent.UserConstructionScript`))