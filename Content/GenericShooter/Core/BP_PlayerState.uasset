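; Player state for GenericShooter that exposes a player's team and ranking score.
; Ranking score is computed from the stat manager component as kills minus suicides and team kills, returned as a float.
; Team functions delegate to the team member component: team change requests go through its server request and always report success, while the setter returns the resulting team number without checking authority itself.
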(fn `GetScoreForRanking`
  (returns (Score :type "Float (double-precision)"))
  (bind _bp_basicstatmanager (`self.BP_BasicStatManager`))
  (bind _statvalue (`/Game/GenericShooter/Addons/StatManager/Core/BP_StatManagerComponent.GetIntStat` _bp_basicstatmanager "Kills" 0))
  (bind _statvalue_2 (`/Game/GenericShooter/Addons/StatManager/Core/BP_StatManagerComponent.GetIntStat` _bp_basicstatmanager "Suicides" 0))
  (bind _statvalue_3 (`/Game/GenericShooter/Addons/StatManager/Core/BP_StatManagerComponent.GetIntStat` _bp_basicstatmanager "TeamKills" 0))
  (return (`KismetMathLibrary.Conv_IntToDouble` (- (- _statvalue _statvalue_2) _statvalue_3))))

(fn `GetTeamNum`
  (returns (TeamNum :type Byte))
  (return (`/Game/GenericShooter/Addons/TeamManager/Core/BP_TeamMemberComponent.GetTeamNum` (`self.BP_TeamMemberComponent`))))

(fn `RequestTeamChange`
  (params (DesiredTeamIndex :type Integer))
  (returns (bRequested :type Boolean))
  (`/Game/GenericShooter/Addons/TeamManager/Core/BP_TeamMemberComponent.ServerRequestTeamChange` (`self.BP_TeamMemberComponent`) self DesiredTeamIndex)
  (return true))

(fn `SetTeamNumIfServer`
  (params (TeamNum :type Byte))
  (returns (NewTeamNum :type Byte))
  (bind _bp_teammembercomponent (`self.BP_TeamMemberComponent`))
  (`/Game/GenericShooter/Addons/TeamManager/Core/BP_TeamMemberComponent.SetTeamNum` _bp_teammembercomponent TeamNum)
  (return (`/Game/GenericShooter/Addons/TeamManager/Core/BP_TeamMemberComponent.GetTeamNum` _bp_teammembercomponent)))

(fn `UserConstructionScript`)